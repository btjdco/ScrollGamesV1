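; Actor component that manages the ability quick slots, binding hotkeys to abilities and activating them on key press.
; Initialize builds one slot object per key of an input action mapping, in reverse order, then restores saved abilities when loading a game.
; Key presses find the matching slot and pass its ability class to the player's AbilityManager.
; It also swaps slot contents, refreshes hotkeys after remapping and returns slot ability classes for saving.
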(fn Initialize
  (bind _manager (Class|BIAbilitySystemActor|GetAbilityManager(Message) (Game|GetPlayerCharacter 0)))
  (Variables|Don'tTouch|SetAbilityManager _manager)
  (Utilities|FlowControl|Sequence
    (:then_0
      (bind _arrayelement (Utilities|Array|ReverseforEachLoop (Class|InputSettings|GetActionMappingbyName (Class|InputSettings|GetInputSettings) (Variables|Settings|GetActionMapping))) ; create empty slots
        (:LoopBody
          (bind _returnvalue (Game|ConstructObjectfromClass self "/Game/AbilitySystem/BP_AbilityQuickSlot.BP_AbilityQuickSlot_C" (Utilities|Struct|BreakInputActionKeyMapping _arrayelement)))
          (Utilities|Array|Add (Variables|Don'tTouch|GetQuickSlots) _returnvalue))))
    (:then_1
      (bind _out (Class|BIGameAbilityGI|IsGameShouldbeLoadedA(Message) (Game|GetGameInstance)))
      (if _out
        (bind _quickslotabilities (Class|BIAbilitySystemSG|GetSavedAbilitySystemData(Message) (CallFunction|GetSaveGameClassALib)))
        (for (_array_element _array_index) _quickslotabilities
          (bind _aability (Default|GetAbilitybyClass (Variables|Don'tTouch|GetAbilityManager) _array_element))
          (Default|UpdateQuickSlot (Utilities|Array|Get(acopy) (Variables|Don'tTouch|GetQuickSlots) _array_index) _aability))))))

(fn SwapSlots
  (params (FromSlot :type BP%20Ability%20Quick%20Slot%20Object%20Reference) (ToSlot :type BP%20Ability%20Quick%20Slot%20Object%20Reference))
  (Variables|/Game/AbilitySystem/BP_AbilityQuickSlot.BP_AbilityQuickSlot_C|GetAbility ToSlot
    (:then
      (LocalVariables|SetlocalAbility (Variables|/Game/AbilitySystem/BP_AbilityQuickSlot.BP_AbilityQuickSlot_C|GetAbility ToSlot)))
    (:else
      _))
  (Default|UpdateQuickSlot ToSlot (Variables|/Game/AbilitySystem/BP_AbilityQuickSlot.BP_AbilityQuickSlot_C|GetAbility FromSlot))
  (Default|UpdateQuickSlot FromSlot (LocalVariables|GetlocalAbility)))

(fn UpdateQuickSlotHotkeys
  (for (_array_element _array_index) (Variables|Don'tTouch|GetQuickSlots)
    (Default|UpdateHotkey _array_element (Variables|Settings|GetActionMapping) (- (Utilities|Array|LastIndex (Variables|Don'tTouch|GetQuickSlots)) _array_index))))

(fn SaveQuickSlots
  (for _array_element (Variables|Don'tTouch|GetQuickSlots)
    (Utilities|Array|Add (LocalVariables|GetlocalQuickSlotAbilities) (Utilities|GetClass (Variables|/Game/AbilitySystem/BP_AbilityQuickSlot.BP_AbilityQuickSlot_C|GetAbility _array_element))))
  (return (LocalVariables|GetlocalQuickSlotAbilities)))

(fn OnPressQuickSlot
  (params (Key :type Key%20Structure :default "None"))
  (bind _quickslot (AbilitySystem|QuickSlotManager|GetQuickSlotbyKey Key))
  (bind _ability (Variables|/Game/AbilitySystem/BP_AbilityQuickSlot.BP_AbilityQuickSlot_C|GetAbility _quickslot)
    (:then
      (Default|TryActivateAbility (Variables|Don'tTouch|GetAbilityManager) (Utilities|GetClass _ability))
      (return))
    (:else)))

(fn GetQuickSlotbyKey
  (params (Key :type Key%20Structure :default "None"))
  (for _array_element (Variables|Don'tTouch|GetQuickSlots)
    (if (== (Variables|/Game/AbilitySystem/BP_AbilityQuickSlot.BP_AbilityQuickSlot_C|GetHotkey _array_element) Key)
      (return _array_element)))
  (return 0))