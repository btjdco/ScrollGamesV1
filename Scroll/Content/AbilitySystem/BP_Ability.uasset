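; Base ability actor that handles activation, costs, cooldown, charges, levels, interruption rules and UI data for its owner's ability manager.
; Activation is gated by cooldown, tags, movement mode, charges and cost, with notifications for most player failures.
; While active, it applies tags through the manager and cancels itself when a blocking tag appears.
; Timers drive cooldown and charge recovery, and save/load restores them, re-activating active passives.
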(event Custom|ActivateAbility
  (Variables|Don'tTouch|SetIsActivated true)
  (Default|ApplyTags (Variables|Don'tTouch|GetOwnerAbilityManager) (Variables|Activation|GetActivationAppliedTags))
  (EventDispatchers|BindEventtoOnApplyTags (Variables|Don'tTouch|GetOwnerAbilityManager) (EventDispatchers|CreateEvent :!event Custom|OnApplyTags)) ; for example, if tag "Stun" or "Silence" is added => ability is canceled
  (Default|CallUpdateUI))

(event Custom|EndAbility
  (Variables|Don'tTouch|SetIsActivated false)
  (Default|RemoveTags (Variables|Don'tTouch|GetOwnerAbilityManager) (Variables|Activation|GetActivationAppliedTags))
  (EventDispatchers|UnbindEventfromOnApplyTags (Variables|Don'tTouch|GetOwnerAbilityManager) (EventDispatchers|CreateEvent :!event Custom|OnApplyTags))
  (Default|AbilityEnded (Variables|Don'tTouch|GetOwnerAbilityManager) self)
  (Default|CallEnd)
  (Default|CallUpdateUI))

(event Custom|CancelAbility
  (if (Variables|Don'tTouch|GetIsActivated)
    (CallFunction|EndAbility)))

(event Custom|OnApplyTags
  (params (Tags :type Gameplay%20Tag%20Container%20Structure))
  (if (GameplayTags|HasAnyTags (Variables|Activation|GetActivationBlockedTags) Tags true) ; If added tag is equal to any blocked tags, ability should be canceled
    (CallFunction|CancelAbility)))

(fn ConstructionScript
  ;[1 1 1] We use construction script instead Begin Play in order to intialize the actor at once upon creation
  ; it is useful, because, sometimes, we spawn actor and make some actions with it, but BeginPlay event hasn't been fired yet
  (Variables|Don'tTouch|SetAbilityOwner (Components|GetOwner))
  (bind _manager (Class|BIAbilitySystemActor|GetAbilityManager(Message) (Variables|Don'tTouch|GetAbilityOwner)))
  (Variables|Don'tTouch|SetOwnerAbilityManager _manager)
  (Variables|Don'tTouch|SetCurrentChargeCount (CallFunction|GetFloatValue (Variables|Charge|GetMaxChargeCount) (Variables|Don'tTouch|GetLevel))))

(fn CanActivateAbility
  (Utilities|FlowControl|Sequence
    (:then_0
      (if (Variables|Don'tTouch|GetInCooldown) ; ability is in cooldown
        (if (AbilitySystem|Ability|Additional|OwnerIsPlayer)
          (Class|BINotificationSystemAbilityController|ShowSystemNotificationA(Message) (Game|GetPlayerController 0) "Ability is in cooldown."))
        (return false)))
    (:then_1
      (if (not (GameplayTags|HasAllTags (Variables|/Game/AbilitySystem/AC_AbilityManager.AC_AbilityManager_C|GetGameplayTags (Variables|Don'tTouch|GetOwnerAbilityManager)) (Variables|Activation|GetActivationRequiredTags) true)) ; Owner has all required tags?
        (if (AbilitySystem|Ability|Additional|OwnerIsPlayer)
          (Class|BINotificationSystemAbilityController|ShowSystemNotificationA(Message) (Game|GetPlayerController 0) "Ability cannot be casted. Caster hasn't all required tags."))
        (return false)))
    (:then_2
      (if (GameplayTags|HasAnyTags (Variables|/Game/AbilitySystem/AC_AbilityManager.AC_AbilityManager_C|GetGameplayTags (Variables|Don'tTouch|GetOwnerAbilityManager)) (Variables|Activation|GetActivationBlockedTags) true) ; stun, silence etc.
        (if (AbilitySystem|Ability|Additional|OwnerIsPlayer)
          (Class|BINotificationSystemAbilityController|ShowSystemNotificationA(Message) (Game|GetPlayerController 0) "Ability cannot be casted. Caster has blocked tags."))
        (return false)))
    (:then_3
      (Utilities|Casting|CastToCharacter (Variables|Don'tTouch|GetAbilityOwner))
      (if (Utilities|Array|ContainsItem (Variables|Activation|GetActivationBlockedMovementModes) (Variables|/Script/Engine.CharacterMovementComponent|GetMovementMode (Variables|/Script/Engine.Character|GetCharacterMovement (.AsCharacter (Utilities|Casting|CastToCharacter (Variables|Don'tTouch|GetAbilityOwner)))))) ; jumping / falling
        (if (AbilitySystem|Ability|Additional|OwnerIsPlayer)
          (Class|BINotificationSystemAbilityController|ShowSystemNotificationA(Message) (Game|GetPlayerController 0) "Ability cannot be casted. Caster is jumping/falling etc."))
        (return false)))
    (:then_4
      (if (AbilitySystem|Ability|Charge|DoUseCharges)
        (if (not (> (Variables|Don'tTouch|GetCurrentChargeCount) 0.0))
          (if (AbilitySystem|Ability|Additional|OwnerIsPlayer)
            (Class|BINotificationSystemAbilityController|ShowSystemNotificationA(Message) (Game|GetPlayerController 0) "Ability cannot be casted. No charges."))
          (return false))))
    (:then_5
      (return (AbilitySystem|Ability|Additional|IsEnoughCost)))))

(fn ApplyCost
  (for _array_element (Variables|Cost|GetCost)
    (Default|ModifyAttribute (Variables|Don'tTouch|GetOwnerAbilityManager) (.Attribute (Utilities|Struct|BreakS_AttributeModificationData _array_element)) (.ValueType (Utilities|Struct|BreakS_AttributeModificationData _array_element)) (.Modifier (Utilities|Struct|BreakS_AttributeModificationData _array_element)) (CallFunction|GetFloatValue (.Value (Utilities|Struct|BreakS_AttributeModificationData _array_element)) (Variables|Don'tTouch|GetLevel)))))

(fn ApplyCooldown
  (if (not (== (CallFunction|GetFloatValue (Variables|Cooldown|GetCooldown) (Variables|Don'tTouch|GetLevel)) 0.0))
    (Variables|Don'tTouch|SetInCooldown true)
    (bind _returnvalue (Utilities|Time|SetTimerbyEvent (EventDispatchers|CreateEvent :!event CooldownExpiration) (CallFunction|GetFloatValue (Variables|Cooldown|GetCooldown) (Variables|Don'tTouch|GetLevel))))
    (Variables|Don'tTouch|SetCooldownTimer _returnvalue)
    (Default|CallUpdateUI)))

(fn CooldownExpiration
  (Variables|Don'tTouch|SetInCooldown false)
  (Utilities|Time|ClearandInvalidateTimerbyHandle (Variables|Don'tTouch|GetCooldownTimer))
  (Default|CallUpdateUI))

(fn GetUIData
  (switch Utilities|FlowControl|Switch|SwitchonE_UIDataSource (Variables|UI|GetUIDataSource)
    (:NewEnumerator0
      (return (Variables|UI|GetUIDataValues)))
    (:NewEnumerator1
      (bind _returnvalue (Utilities|GetDataTableRow (Variables|UI|GetUIDataTable) (Utilities|String|StringToName (Utilities|String|ToString(Integer) (Variables|Don'tTouch|GetLevel))))
        (:then
          (return _returnvalue))))))

(fn IsPassive
  (return (GameplayTags|HasTag (Variables|Ability|GetAbilityTags) "(TagName=\"Ability.Passive\")" true)))

(fn LevelUp
  (if (not (AbilitySystem|Ability|Level|IsMaxLevel))
    (Math|Integer|IncrementInt (Variables|Don'tTouch|GetLevel)
      (:%20%20
        (Default|CallUpdateUI)))))

(fn ResetLevel
  (Variables|Don'tTouch|SetLevel 1)
  (Default|CallUpdateUI))

(fn IsMaxLevel
  (return (== (Variables|Don'tTouch|GetLevel) (Variables|Ability|GetMaxLevel))))

(fn ModifyCharge
  (params (Amount :type Float%20%28double-precision%29))
  (Variables|Don'tTouch|SetCurrentChargeCount (Math|Float|Clamp(Float) (+ (Variables|Don'tTouch|GetCurrentChargeCount) Amount) 0.0 (CallFunction|GetFloatValue (Variables|Charge|GetMaxChargeCount) (Variables|Don'tTouch|GetLevel))))
  (Default|CallUpdateUI)
  (if (== (Variables|Don'tTouch|GetCurrentChargeCount) (CallFunction|GetFloatValue (Variables|Charge|GetMaxChargeCount) (Variables|Don'tTouch|GetLevel)))
    (return)
    (else
      (switch Utilities|FlowControl|Switch|SwitchonE_ChargeRecoveryPolicy (Variables|Charge|GetChargeRecoveryPolicy)
        (:NewEnumerator0
          (bind _returnvalue (Utilities|Time|SetTimerbyEvent (EventDispatchers|CreateEvent :!event RecoveryCharge) (CallFunction|GetFloatValue (Variables|Charge|GetChargeRecoveryTime) (Variables|Don'tTouch|GetLevel))))
          (Variables|Don'tTouch|SetChargeRecoveryTimer _returnvalue))
        (:NewEnumerator1
          (return))))))

(fn DoUseCharges
  (return (> (CallFunction|GetFloatValue (Variables|Charge|GetMaxChargeCount) (Variables|Don'tTouch|GetLevel)) 0.0)))

(fn RecoveryCharge
  (AbilitySystem|Ability|Charge|ModifyCharge 1.0))

(fn IsEnoughCost
  (for _array_element (Variables|Cost|GetCost)
    (LocalVariables|SetlocalCost _array_element)
    (LocalVariables|SetlocalAttribute (Default|GetAttribute (Variables|Don'tTouch|GetOwnerAbilityManager) (Utilities|Struct|BreakS_AttributeModificationData (LocalVariables|GetlocalCost))))
    (switch Utilities|FlowControl|Switch|SwitchonE_Modifier (Utilities|Struct|BreakS_AttributeModificationData (LocalVariables|GetlocalCost))
      (:NewEnumerator1
        (if (not (>= (Variables|/Game/AbilitySystem/BP_Attribute.BP_Attribute_C|GetCurrentValue (LocalVariables|GetlocalAttribute)) (CallFunction|GetFloatValue (Utilities|Struct|BreakS_AttributeModificationData (LocalVariables|GetlocalCost)) (Variables|Don'tTouch|GetLevel))))
          (return false)))
      (:NewEnumerator3
        (if (not (>= (Variables|/Game/AbilitySystem/BP_Attribute.BP_Attribute_C|GetCurrentValue (LocalVariables|GetlocalAttribute)) (* (Variables|/Game/AbilitySystem/BP_Attribute.BP_Attribute_C|GetRealValue (LocalVariables|GetlocalAttribute)) (CallFunction|GetFloatValue (Utilities|Struct|BreakS_AttributeModificationData (LocalVariables|GetlocalCost)) (Variables|Don'tTouch|GetLevel)))))
          (return false)))))
  (return true))

(fn SaveAbility
  (return (Utilities|Struct|MakeS_SavedAbility (Utilities|GetClass self) (Variables|Don'tTouch|GetLevel) (Variables|Don'tTouch|GetCurrentChargeCount) (Utilities|Time|GetTimerRemainingTimebyHandle (Variables|Don'tTouch|GetCooldownTimer)) (Utilities|Time|GetTimerRemainingTimebyHandle (Variables|Don'tTouch|GetChargeRecoveryTimer)) (Variables|Don'tTouch|GetIsActivated))))

(fn LoadAbility
  (params (SavedAbility :type S%20Saved%20Ability%20Structure))
  (Utilities|FlowControl|Sequence
    (:then_0
      (Variables|Don'tTouch|SetCurrentChargeCount (.currentcharges SavedAbility)))
    (:then_1
      (if (> (.remainingchargerecoverytime SavedAbility) 0.0) ; charges are recovering?
        (bind _returnvalue (Utilities|Time|SetTimerbyEvent (EventDispatchers|CreateEvent :!event RecoveryCharge) (.remainingchargerecoverytime SavedAbility)))
        (Variables|Don'tTouch|SetChargeRecoveryTimer _returnvalue)))
    (:then_2
      (if (> (.remainingcooldowntime SavedAbility) 0.0) ; is in cooldown?
        (Variables|Don'tTouch|SetInCooldown true)
        (bind _returnvalue_2 (Utilities|Time|SetTimerbyEvent (EventDispatchers|CreateEvent :!event CooldownExpiration) (.remainingcooldowntime SavedAbility)))
        (Variables|Don'tTouch|SetCooldownTimer _returnvalue_2)))
    (:then_3
      (Default|CallUpdateUI)
      (if (and (AbilitySystem|Ability|Additional|IsPassive) (.isactivated SavedAbility))
        (Default|TryActivateAbility (Variables|Don'tTouch|GetOwnerAbilityManager) (Utilities|GetClass self))))))

(fn CanbeInterruptedbyAbility
  (params (Ability :type BP%20Ability%20Class%20Reference))
  (switch Utilities|FlowControl|Switch|SwitchonE_InterruptionPolicy (Variables|Interruption|GetInterruptionPolicy)
    (:NewEnumerator0
      (return true))
    (:NewEnumerator3
      (return (Utilities|Array|ContainsItem (Variables|Interruption|GetInterruptionList) Ability)))
    (:NewEnumerator1
      (return (not (Utilities|Array|ContainsItem (Variables|Interruption|GetInterruptionList) Ability))))))

(fn CalcAnimationPlayRate
  (LocalVariables|SetlocalAttribute (Default|GetAttribute (Variables|Don'tTouch|GetOwnerAbilityManager) "NewEnumerator43"))
  (LocalVariables|GetlocalAttribute
    (:then
      (return (Variables|/Game/AbilitySystem/BP_Attribute.BP_Attribute_C|GetRealValue (LocalVariables|GetlocalAttribute))))
    (:else
      (return 1.0))))

(fn OwnerIsPlayer
  (return (== (Variables|Don'tTouch|GetAbilityOwner) (Game|GetPlayerCharacter 0))))