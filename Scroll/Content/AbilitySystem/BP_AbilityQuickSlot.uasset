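; Ability system quick slot Blueprint that holds an assigned ability and a hotkey for it.
; UpdateQuickSlot stores the given ability and calls the UI update.
; UpdateHotkey looks up the key at a given index among an input action's mappings in Input Settings, stores it and calls the hotkey UI update.
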(fn UpdateQuickSlot
  (params (Ability :type BP%20Ability%20Object%20Reference))
  (Variables|Default|SetAbility Ability)
  (Default|CallUpdateUI))

(fn UpdateHotkey
  (params (Action :type Name) (Index :type Integer))
  (Variables|Default|SetHotkey (Utilities|Struct|BreakInputActionKeyMapping (Utilities|Array|Get(acopy) (Class|InputSettings|GetActionMappingbyName (Class|InputSettings|GetInputSettings) Action) Index)))
  (Default|CallUpdateHotkeyUI))