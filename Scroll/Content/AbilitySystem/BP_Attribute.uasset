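; Attribute object in the ability system that holds one stat's base, real, current and blocked values and restores them on load.
; Modify adds, subtracts or adjusts by percentage, deriving real value from base and an additive multiplier and capping current by the unblocked share.
; Base changes propagate the real-value delta to dependent attributes through AbilityManager.
; One attribute type also writes its real value to the outer Character's MaxWalkSpeed.
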(fn Modify
  (params (AttributeValue :type E_AttributeValue%20Enum :default "NewEnumerator0") (Modifier :type E_Modifier%20Enum :default "NewEnumerator0") (Value :type Float%20%28double-precision%29))
  (LocalVariables|SetlocalOldRealValue (Variables|Default|GetRealValue))
  (switch Utilities|FlowControl|Switch|SwitchonE_AttributeValue AttributeValue
    (:NewEnumerator0
      ;[1 1 1] Base
      (switch Utilities|FlowControl|Switch|SwitchonE_Modifier Modifier
        (:NewEnumerator0
          (Variables|Default|SetBaseValue (+ (Variables|Default|GetBaseValue) Value)))
        (:NewEnumerator1
          (Variables|Default|SetBaseValue (- (Variables|Default|GetBaseValue) Value)))
        (:NewEnumerator2
          (Variables|Default|SetMultiplier (+ (Variables|Default|GetMultiplier) Value))
          (if (Math|Float|NearlyEqual(Float) (Variables|Default|GetMultiplier) 0.0 1e-06) :!label _label
            (Variables|Default|SetMultiplier 0.0) ; useful to convert -0 to 0
          ))
        (:NewEnumerator3
          (Variables|Default|SetMultiplier (- (Variables|Default|GetMultiplier) Value))
          (goto _label)))
      (Variables|Default|SetRealValue (Math|Float|Clamp(Float) (+ (Variables|Default|GetBaseValue) (* (Variables|Default|GetBaseValue) (Variables|Default|GetMultiplier))) (Variables|Attribute|GetMinValue) (Variables|Attribute|GetMaxValue)))
      (Variables|Default|SetCurrentValue (Math|Float|Clamp(Float) (Variables|Default|GetCurrentValue) (Variables|Attribute|GetMinValue) (- (Variables|Default|GetRealValue) (* (Variables|Default|GetRealValue) (Variables|Default|GetBlockedValue))))) ; useful when quickly decreasing real value\nin this case current value shouln't be greater than real value
      (Default|CallOnModify)
      (CallFunction|UpdateMovementSpeed)
      (for _array_element (Variables|Advanced|GetAffectsAttributes)
        (Default|ModifyAttribute (Variables|Default|GetAbilityManager) (.Attribute (Utilities|Struct|BreakS_AttributeModificationData _array_element)) "NewEnumerator0" (.Modifier (Utilities|Struct|BreakS_AttributeModificationData _array_element)) (* (.Value (Utilities|Struct|BreakS_FloatValue (.Value (Utilities|Struct|BreakS_AttributeModificationData _array_element)))) (- (Variables|Default|GetRealValue) (LocalVariables|GetlocalOldRealValue))))))
    (:NewEnumerator1
      ;[1 1 1] Current
      (switch Utilities|FlowControl|Switch|SwitchonE_Modifier Modifier
        (:NewEnumerator0
          (Variables|Default|SetCurrentValue (+ (Variables|Default|GetCurrentValue) Value)))
        (:NewEnumerator1
          (Variables|Default|SetCurrentValue (- (Variables|Default|GetCurrentValue) Value)))
        (:NewEnumerator2
          (Variables|Default|SetCurrentValue (+ (Variables|Default|GetCurrentValue) (* (Variables|Default|GetRealValue) Value))))
        (:NewEnumerator3
          (Variables|Default|SetCurrentValue (- (Variables|Default|GetCurrentValue) (* (Variables|Default|GetRealValue) Value)))))
      (Variables|Default|SetCurrentValue (Math|Float|Clamp(Float) (Variables|Default|GetCurrentValue) (Variables|Attribute|GetMinValue) (- (Variables|Default|GetRealValue) (* (Variables|Default|GetRealValue) (Variables|Default|GetBlockedValue)))))
      (Default|CallOnModify))
    (:NewEnumerator2
      ;[1 1 1] Blocked
      (switch Utilities|FlowControl|Switch|SwitchonE_Modifier Modifier
        (:NewEnumerator0
          (Variables|Default|SetBlockedValue (+ (Variables|Default|GetBlockedValue) Value)))
        (:NewEnumerator1
          (Variables|Default|SetBlockedValue (- (Variables|Default|GetBlockedValue) Value)))
        (:NewEnumerator2
          ;;[1 1 1] Just in case. But you need to use Add or Subtruct. It won't work in most cases because blocked value almost always is equal to 0
          (Variables|Default|SetBlockedValue (+ (Variables|Default|GetBlockedValue) (* (Variables|Default|GetBlockedValue) Value))))
        (:NewEnumerator3
          (Variables|Default|SetBlockedValue (- (Variables|Default|GetBlockedValue) (* (Variables|Default|GetBlockedValue) Value)))))
      (Variables|Default|SetBlockedValue (Math|Float|Clamp(Float) (Variables|Default|GetBlockedValue)))
      (Variables|Default|SetCurrentValue (Math|Float|Clamp(Float) (Variables|Default|GetCurrentValue) (Variables|Attribute|GetMinValue) (- (Variables|Default|GetRealValue) (* (Variables|Default|GetRealValue) (Variables|Default|GetBlockedValue)))))
      (Default|CallOnModify))))

(fn Load
  (params (CurrentValue :type Float%20%28double-precision%29) (RealValue :type Float%20%28double-precision%29) (BlockedValue :type Float%20%28double-precision%29) (BaseValue :type Float%20%28double-precision%29) (Multiplier :type Float%20%28double-precision%29))
  (Variables|Default|SetCurrentValue CurrentValue)
  (Variables|Default|SetRealValue RealValue)
  (Variables|Default|SetBlockedValue BlockedValue)
  (Variables|Default|SetBaseValue BaseValue)
  (Variables|Default|SetMultiplier Multiplier)
  (CallFunction|UpdateMovementSpeed))

(fn UpdateMovementSpeed
  (if (Utilities|Enum|Equal(Enum) (Variables|Attribute|GetAttribute) "NewEnumerator21")
    (bind _ascharacter (Utilities|Casting|CastToCharacter (Utilities|GetOuterObject self)))
    (Variables|/Script/Engine.CharacterMovementComponent|SetMaxWalkSpeed (Variables|/Script/Engine.Character|GetCharacterMovement _ascharacter) (Variables|Default|GetRealValue))))