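; BP_Effect is a gameplay effect object that changes attributes, tags, abilities and nested effects through its owning ability manager.
; Apply runs modifiers, executions and FX once or on a looping tick timer, which tags can block.
; Stacking uses shared or per-stack duration timers with configurable expiration.
; Removal inverts non-periodic modifiers and keeps tags other effects grant; stacks and remaining time support save/load, and values can scale by level through curve tables.
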(fn Apply
  (bind _manager (Class|BIAbilitySystemActor|GetAbilityManager(Message) (Utilities|GetOuterObject self)))
  (Variables|Default|SetOwnerAbilityManager _manager)
  (Utilities|FlowControl|Sequence
    (:then_0
      (if (AbilitySystem|Effect|Additional|IsTemporary)
        (AbilitySystem|Effect|Duration|HandleDuration)))
    (:then_1
      ;[1 1 1] Tags and Abilities are not applied on tick
      (Default|ApplyTags (Variables|Default|GetOwnerAbilityManager) (Variables|Effect|GetAppliedTags))
      (AbilitySystem|Effect|Application|ApplyAbilities))
    (:then_2
      (if (AbilitySystem|Effect|Additional|IsPeriodic)
        (AbilitySystem|Effect|Duration|CreateTickTimer)
        (for _array_element (Variables|Effect|GetExecutions)
          (bind _out (AbilitySystem|Effect|Application|CreateExecution _array_element))
          (Utilities|Array|Add (Variables|Default|GetTickExecutions) _out))
        (if (Variables|Tick|GetExecuteOnApplication)
          (AbilitySystem|Effect|Application|ApplyonTick))
        (else
          (AbilitySystem|Effect|Application|ApplyModifiers)
          (AbilitySystem|Effect|Application|ApplyEffects)
          (for _array_element_2 (Variables|Effect|GetExecutions)
            (bind _out_2 (AbilitySystem|Effect|Application|CreateExecution _array_element_2))
            (Default|Execute _out_2)))))
    (:then_3
      (AbilitySystem|Effect|Application|SpawnFX (Variables|Visual|GetOnApplicationFX)))))

(fn ApplyOverflowEffects
  (for _array_element (Variables|Stack|GetOverflowEffects)
    (Default|ApplyEffect (Variables|Default|GetOwnerAbilityManager) (Utilities|Struct|MakeS_EffectData (.Effect (Utilities|Struct|BreakS_EffectData _array_element)) (.Level (Utilities|Struct|BreakS_EffectData _array_element)) (Variables|Default|GetCauser) (.UseOverrideData (Utilities|Struct|BreakS_EffectData _array_element)) (.OverrideData (Utilities|Struct|BreakS_EffectData _array_element)) false "0.000000,0.000000,0.000000"))))

(fn OverrideData
  (params (Data :type S%20Effect%20Override%20Data%20Structure))
  (Variables|Tick|SetTick (.tick Data))
  (Variables|Application|SetChanceToApply (.chancetoapply Data))
  (Variables|Duration|SetDuration (.duration Data))
  (Variables|Duration|SetDurationPolicy (.durationpolicy Data))
  (Variables|Duration|SetExpirationPolicy (.expirationpolicy Data)))

(fn Remove
  (Utilities|FlowControl|Sequence
    (:then_0
      ;[1 1 1] Clear all timers
      (Utilities|Time|ClearTimerbyFunctionName 0 (Variables|Default|GetDurationTimerFunctionName))
      (Utilities|Time|ClearTimerbyFunctionName 0 (Variables|Default|GetTickTimerFunctionName))
      (for _array_element (Variables|Default|GetDurationTimers)
        (Default|Stop _array_element)))
    (:then_1
      ;[1 1 1] Remove all visual effects
      (for _array_element_2 (Variables|Default|GetSpawnedFX)
        (Default|Remove _array_element_2))
      (Utilities|Array|Clear (Variables|Default|GetSpawnedFX)))
    (:then_2
      (Utilities|FlowControl|Sequence
        (:then_0
          ;[1 1 1] Since Abilities and Tags are applied only one time, it makes sense to remove them also one time
          (for _array_element_3 (Variables|Effect|GetAppliedAbilities)
            (Default|RemoveAbility (Variables|Default|GetOwnerAbilityManager) _array_element_3)))
        (:then_1
          (for _array_element_4 (.gameplaytags (Variables|Effect|GetAppliedTags))
            (if (AbilitySystem|Effect|Additional|ShouldRemoveTag _array_element_4)
              (Default|RemoveTags (Variables|Default|GetOwnerAbilityManager) (Utilities|Struct|MakeGameplayTagContainer (Utilities|Array|MakeArray _array_element_4))))))
        (:then_2
          (if (not (AbilitySystem|Effect|Additional|IsPeriodic)) ; it is supposed that periodic effects modify current values, not base, so we don't need to restore the values
            (for _index (range 1 (Variables|Default|GetStackCount))
              (for _array_element_5 (Variables|Effect|GetAppliedModifiers)
                (Default|ModifyAttribute (Variables|Default|GetOwnerAbilityManager) (.Attribute (Utilities|Struct|BreakS_AttributeModificationData _array_element_5)) (.ValueType (Utilities|Struct|BreakS_AttributeModificationData _array_element_5)) (Utilities|Select :Index (.Modifier (Utilities|Struct|BreakS_AttributeModificationData _array_element_5)) :NewEnumerator0 "NewEnumerator1" :NewEnumerator1 "NewEnumerator0" :NewEnumerator2 "NewEnumerator3" :NewEnumerator3 "NewEnumerator2") (AbilitySystem|Effect|Additional|GetFloatValue (.Value (Utilities|Struct|BreakS_AttributeModificationData _array_element_5))))))))))))

(fn ApplyonTick
  (if (AbilitySystem|Effect|Application|CanApplyonTick)
    (AbilitySystem|Effect|Application|SpawnFX (Variables|Visual|GetOnTickFX))
    (Utilities|FlowControl|Sequence
      (:then_0
        (for _index (range 1 (Variables|Default|GetStackCount))
          (Utilities|FlowControl|Sequence
            (:then_0
              (AbilitySystem|Effect|Application|ApplyModifiers))
            (:then_1
              (AbilitySystem|Effect|Application|ApplyEffects)))))
      (:then_1
        (if (Variables|Tick|GetPerformExecutionOnlyOnce)
          (for _array_element (Variables|Default|GetTickExecutions) :!label _label ; We don't need to create execution object classes on each tick\ncreate one time, on effect application, and then just execute them
            (Default|Execute _array_element))
          (else
            (for _index_2 (range 1 (Variables|Default|GetStackCount))
              (goto _label))))))))

(fn CanApplyonTick
  (return (not (GameplayTags|HasAnyTags (Variables|/Game/AbilitySystem/AC_AbilityManager.AC_AbilityManager_C|GetGameplayTags (Variables|Default|GetOwnerAbilityManager)) (Variables|Tick|GetTickApplicationBlockedTags) true))))

(fn ApplyModifiers
  (for _array_element (Variables|Effect|GetAppliedModifiers)
    (Default|ModifyAttribute (Variables|Default|GetOwnerAbilityManager) (.Attribute (Utilities|Struct|BreakS_AttributeModificationData _array_element)) (.ValueType (Utilities|Struct|BreakS_AttributeModificationData _array_element)) (.Modifier (Utilities|Struct|BreakS_AttributeModificationData _array_element)) (AbilitySystem|Effect|Additional|GetFloatValue (.Value (Utilities|Struct|BreakS_AttributeModificationData _array_element))))))

(fn ApplyEffects
  (for _array_element (Variables|Effect|GetAppliedEffects)
    (Default|ApplyEffect (Variables|Default|GetOwnerAbilityManager) (Utilities|Struct|MakeS_EffectData _array_element (Variables|Default|GetLevel) (Variables|Default|GetCauser) false "(Tick_17_40755E2C4DCAD94CF3DBA2AECC805C15=(Source_10_0C1CA74C4C120C42C1F857BD53F0A76F=NewEnumerator0,Value_5_90E89AB144D6F3B57A2FB59966A03498=0.000000,CurveTable_11_2B4B079B4C7ECA70D04E3F947A964B45=(CurveTable=None,RowName=\"\")),ChanceToApply_19_3C8E08B246FF3BA8A2CDA8A8D9F764C6=(Source_10_0C1CA74C4C120C42C1F857BD53F0A76F=NewEnumerator0,Value_5_90E89AB144D6F3B57A2FB59966A03498=0.000000,CurveTable_11_2B4B079B4C7ECA70D04E3F947A964B45=(CurveTable=None,RowName=\"\")),Duration_29_7F8704364211410D0930AD8AB240975B=(Source_10_0C1CA74C4C120C42C1F857BD53F0A76F=NewEnumerator0,Value_5_90E89AB144D6F3B57A2FB59966A03498=0.000000,CurveTable_11_2B4B079B4C7ECA70D04E3F947A964B45=(CurveTable=None,RowName=\"\")),DurationPolicy_32_683FC34B46CBA1C769699589F12C9837=NewEnumerator1,ExpirationPolicy_36_54D3E72548F23CD877ABE988E2FC308D=NewEnumerator0)" false "0.000000,0.000000,0.000000"))))

(fn ApplyAbilities
  (for _array_element (Variables|Effect|GetAppliedAbilities)
    (Default|GiveAbility (Variables|Default|GetOwnerAbilityManager) _array_element (Variables|Default|GetLevel))
    (Default|TryActivateAbility (Variables|Default|GetOwnerAbilityManager) _array_element)))

(fn CreateExecution
  (params (Execution :type BP%20Execution%20Class%20Reference))
  (bind _ownerabilitymanager (Variables|Default|GetOwnerAbilityManager))
  (bind _returnvalue (Components|GetOwner _ownerabilitymanager))
  (bind _returnvalue_2 (Game|ConstructObjectfromClass _returnvalue Execution _returnvalue (Variables|Default|GetCauser) self 0 (Variables|Default|GetLevel)))
  (return _returnvalue_2))

(fn OnExpired
  (switch Utilities|FlowControl|Switch|SwitchonE_DurationPolicy (Variables|Duration|GetDurationPolicy)
    (:NewEnumerator1
      (switch Utilities|FlowControl|Switch|SwitchonE_ExpirationPolicy (Variables|Duration|GetExpirationPolicy) :!label _label
        (:NewEnumerator0
          (if (> (Variables|Default|GetStackCount) 1)
            (AbilitySystem|Effect|Stack|RemoveStack)
            (AbilitySystem|Effect|Duration|CreateDurationTimer (AbilitySystem|Effect|Additional|GetFloatValue (Variables|Duration|GetDuration)))
            (else
              (Default|RemoveEffectbyClass (Variables|Default|GetOwnerAbilityManager) (Utilities|GetClass self) :!label _label_2))))
        (:NewEnumerator1
          (goto _label_2))))
    (:NewEnumerator0
      (if (> (Variables|Default|GetStackCount) 1)
        (AbilitySystem|Effect|Stack|RemoveStack)
        (else
          (Default|RemoveEffectbyClass (Variables|Default|GetOwnerAbilityManager) (Utilities|GetClass self)))))
    (:NewEnumerator2
      (goto _label))))

(fn GetFloatValue
  (params (Parameter :type S%20Float%20Value%20Structure))
  (bind (_curvetable _rowname) (Utilities|Struct|BreakCurveTableRowHandle (.curvetable Parameter)))
  (switch Utilities|FlowControl|Switch|SwitchonE_FloatValueSource (.source Parameter)
    (:NewEnumerator0
      (return (.value Parameter)))
    (:NewEnumerator1
      (bind _outxy (DataTable|EvaluateCurveTableRow _curvetable _rowname (Math|Conversions|ToFloat(Integer) (Variables|Default|GetLevel)))
        (:RowFound
          (return _outxy))))))

(fn IsTemporary
  (return (> (AbilitySystem|Effect|Additional|GetFloatValue (Variables|Duration|GetDuration)) 0.0)))

(fn IsPeriodic
  (return (> (AbilitySystem|Effect|Additional|GetFloatValue (Variables|Tick|GetTick)) 0.0)))

(fn AddStack
  (Math|Integer|IncrementInt (Variables|Default|GetStackCount) ; +1 to stack count
    (:%20%20
      (Default|CallUpdateUI)
      (Utilities|FlowControl|Sequence
        (:then_0
          (if (AbilitySystem|Effect|Additional|IsTemporary)
            (AbilitySystem|Effect|Duration|HandleDuration)))
        (:then_1
          (if (Variables|Visual|GetSpawnOnEachStack) ; apply vis effect on each stack?
            (AbilitySystem|Effect|Application|SpawnFX (Variables|Visual|GetOnApplicationFX))))
        (:then_2
          (if (not (AbilitySystem|Effect|Additional|IsPeriodic))
            (AbilitySystem|Effect|Application|ApplyModifiers)
            (AbilitySystem|Effect|Application|ApplyEffects)
            (for _array_element (Variables|Effect|GetExecutions)
              (bind _out (AbilitySystem|Effect|Application|CreateExecution _array_element))
              (Default|Execute _out))))))))

(fn RemoveStack
  (Math|Integer|DecrementInt (Variables|Default|GetStackCount)
    (:%20%20
      (Default|CallUpdateUI)
      (Utilities|FlowControl|Sequence
        (:then_0
          (if (and (AbilitySystem|Effect|Additional|IsTemporary) (Utilities|Enum|Equal(Enum) (Variables|Duration|GetDurationPolicy) "NewEnumerator0"))
            (Utilities|Array|RemoveIndex (Variables|Default|GetDurationTimers)) ; always the first stack's timer is expired
          ))
        (:then_1
          (if (not (AbilitySystem|Effect|Additional|IsPeriodic))
            (for _array_element (Variables|Effect|GetAppliedModifiers)
              (Default|ModifyAttribute (Variables|Default|GetOwnerAbilityManager) (.Attribute (Utilities|Struct|BreakS_AttributeModificationData _array_element)) (.ValueType (Utilities|Struct|BreakS_AttributeModificationData _array_element)) (Utilities|Select :Index (.Modifier (Utilities|Struct|BreakS_AttributeModificationData _array_element)) :NewEnumerator0 "NewEnumerator1" :NewEnumerator1 "NewEnumerator0" :NewEnumerator2 "NewEnumerator3" :NewEnumerator3 "NewEnumerator2") (AbilitySystem|Effect|Additional|GetFloatValue (.Value (Utilities|Struct|BreakS_AttributeModificationData _array_element)))))))))))

(fn IsStackable
  (return (> (Variables|Stack|GetStackLimitCount) 1)))

(fn IsStackOverflow
  (return (== (Variables|Default|GetStackCount) (Variables|Stack|GetStackLimitCount))))

(fn ShouldRemoveTag
  (params (Tag :type Gameplay%20Tag%20Structure))
  (bind _effects (Default|GetAllAppliedEffects (Variables|Default|GetOwnerAbilityManager)))
  (for _array_element _effects
    (if (and (!= _array_element self) (GameplayTags|HasTag (Variables|BP_Effect_C|GetAppliedTags _array_element) Tag true))
      (return false)))
  (return true))

(fn GetUIData
  (switch Utilities|FlowControl|Switch|SwitchonE_UIDataSource (Variables|GUI|GetUIDataSource)
    (:NewEnumerator0
      (return (Variables|GUI|GetUIDataValues)))
    (:NewEnumerator1
      (bind _returnvalue (Utilities|GetDataTableRow (Variables|GUI|GetUIDataTable) (Utilities|String|StringToName (Utilities|String|ToString(Integer) (Variables|Default|GetLevel))))
        (:then
          (return _returnvalue))))))

(fn GetRemainingDuration
  (return (Class|KismetSystemLibrary|GetTimerRemainingTime 0 (Variables|Default|GetDurationTimerFunctionName))))

(fn SaveEffect
  (if (AbilitySystem|Effect|Additional|IsTemporary)
    (switch Utilities|FlowControl|Switch|SwitchonE_DurationPolicy (Variables|Duration|GetDurationPolicy)
      (:NewEnumerator1
        _)
      (:NewEnumerator0
        (for _array_element (Variables|Default|GetDurationTimers) ; save timers for each stack
          (Utilities|Array|Add (LocalVariables|GetlocalDurationTimers) (Default|GetRemainingTime _array_element)))
        (return (Utilities|Struct|MakeS_SavedEffect (Utilities|GetClass self) (Variables|Default|GetStackCount) (LocalVariables|GetlocalDurationTimers) (Variables|Default|GetLevel))))
      (:NewEnumerator2
        _))
    (return (Utilities|Struct|MakeS_SavedEffect (Utilities|GetClass self) (Variables|Default|GetStackCount) (AbilitySystem|Effect|Additional|GetRemainingDuration) (Variables|Default|GetLevel)))
    (else
      (return (Utilities|Struct|MakeS_SavedEffect (Utilities|GetClass self) (Variables|Default|GetStackCount) (Variables|Default|GetLevel))))))

(fn LoadEffect
  (params (SavedEffect :type S%20Saved%20Effect%20Structure%20%28by%20ref%29))
  (bind _manager (Class|BIAbilitySystemActor|GetAbilityManager(Message) (Utilities|GetOuterObject self)))
  (Variables|Default|SetOwnerAbilityManager _manager)
  (Variables|Default|SetStackCount (Utilities|Struct|BreakS_SavedEffect SavedEffect))
  (Default|CallUpdateUI)
  (Utilities|FlowControl|Sequence
    (:then_0
      (if (AbilitySystem|Effect|Additional|IsTemporary) ; Is Temporary
        (switch Utilities|FlowControl|Switch|SwitchonE_DurationPolicy (Variables|Duration|GetDurationPolicy)
          (:NewEnumerator1
            (AbilitySystem|Effect|Duration|CreateDurationTimer (.durationtimer SavedEffect) :!label _label))
          (:NewEnumerator0
            (for _array_element (Utilities|Struct|BreakS_SavedEffect SavedEffect)
              (bind _returnvalue (Game|ConstructObjectfromClass self "/Game/AbilitySystem/BP_Timer.BP_Timer_C"))
              (Utilities|Array|Add (Variables|Default|GetDurationTimers) _returnvalue)
              (Default|Start _returnvalue _array_element)
              (EventDispatchers|BindEventtoOnExpired _returnvalue (EventDispatchers|CreateEvent :!event OnExpired))))
          (:NewEnumerator2
            (goto _label)))))
    (:then_1
      (for _array_element_2 (Variables|Effect|GetExecutions)
        (bind _out (AbilitySystem|Effect|Application|CreateExecution _array_element_2))
        (Utilities|Array|Add (Variables|Default|GetTickExecutions) _out)))
    (:then_2
      (if (AbilitySystem|Effect|Additional|IsPeriodic) ; Has Tick
        (AbilitySystem|Effect|Duration|CreateTickTimer)))
    (:then_3
      (for _array_element_3 (Variables|Visual|GetOnApplicationFX)
        (if (Utilities|GetClassDefaults _array_element_3)
          (Utilities|Array|Add (LocalVariables|GetlocalFX) _array_element_3)))
      (AbilitySystem|Effect|Application|SpawnFX (LocalVariables|GetlocalFX)))))

(fn CreateDurationTimer
  (params (Time :type Float%20%28double-precision%29))
  (Utilities|Time|SetTimerbyFunctionName 0 (Variables|Default|GetDurationTimerFunctionName) Time))

(fn RefreshDurationTimer
  (Utilities|Time|SetTimerbyFunctionName 0 (Variables|Default|GetDurationTimerFunctionName) (AbilitySystem|Effect|Additional|GetFloatValue (Variables|Duration|GetDuration))))

(fn CreateTickTimer
  (Utilities|Time|SetTimerbyFunctionName 0 (Variables|Default|GetTickTimerFunctionName) (AbilitySystem|Effect|Additional|GetFloatValue (Variables|Tick|GetTick)) true))

(fn HandleDuration
  (switch Utilities|FlowControl|Switch|SwitchonE_DurationPolicy (Variables|Duration|GetDurationPolicy)
    (:NewEnumerator1
      (AbilitySystem|Effect|Duration|CreateDurationTimer (AbilitySystem|Effect|Additional|GetFloatValue (Variables|Duration|GetDuration)) :!label _label) ; Create or Refresh timer
    )
    (:NewEnumerator0
      (bind _returnvalue (Game|ConstructObjectfromClass self "/Game/AbilitySystem/BP_Timer.BP_Timer_C"))
      (Utilities|Array|Add (Variables|Default|GetDurationTimers) _returnvalue)
      (Default|Start _returnvalue (AbilitySystem|Effect|Additional|GetFloatValue (Variables|Duration|GetDuration)))
      (EventDispatchers|BindEventtoOnExpired _returnvalue (EventDispatchers|CreateEvent :!event OnExpired)))
    (:NewEnumerator2
      (if (not (Class|KismetSystemLibrary|TimerExists 0 (Variables|Default|GetDurationTimerFunctionName)))
        (goto _label)))))

(fn SpawnFX
  (params (FX :type Array%20of%20BP%20FX%20Class%20References))
  (for _array_element FX
    (bind _returnvalue (Game|ConstructObjectfromClass self _array_element (Utilities|Struct|MakeS_FXData (Components|GetOwner (Variables|Default|GetOwnerAbilityManager)) (Variables|Default|GetCauser) (Variables|Default|GetLevel))))
    (Default|Execute _returnvalue)
    (Utilities|Array|Add (Variables|Default|GetSpawnedFX) _returnvalue)))

(fn GetSpecialValue
  (return 0.0))