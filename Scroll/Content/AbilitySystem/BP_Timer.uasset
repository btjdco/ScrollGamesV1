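; BP_Timer is a Blueprint timer wrapper in the AbilitySystem folder that offers start, stop and remaining-time queries.
; Start, Stop and GetRemainingTime set, clear and read an engine timer by the function name held in ExpiredFunctionName.
; The Expired function calls OnExpired to signal completion.
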(fn Start
  (params (Time :type Float%20%28double-precision%29))
  (Utilities|Time|SetTimerbyFunctionName 0 (Variables|Default|GetExpiredFunctionName) Time))

(fn Expired
  (Default|CallOnExpired))

(fn GetRemainingTime
  (return (Class|KismetSystemLibrary|GetTimerRemainingTime 0 (Variables|Default|GetExpiredFunctionName))))

(fn Stop
  (Utilities|Time|ClearTimerbyFunctionName 0 (Variables|Default|GetExpiredFunctionName)))