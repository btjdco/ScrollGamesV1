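; Actor component that manages a character's weapon equipment slots and switches between weapon modes.
; Initialize builds slot objects from configured data; equipping replaces the first type-matching slot's item and spawns its weapon actor.
; Weapon modes map to slot indices, whose activation toggles weapon callbacks and reattaches weapons between active and inactive mesh sockets.
; A tag query detects another active weapon sharing a tag for dual-wielding, and EndPlay destroys all spawned weapons.
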(event EventEndPlay
  (params (EndPlayReason :type EEndPlayReason%20Enum :default "Destroyed"))
  (for _array_element (Variables|Don'tTouch|GetSlots) ; destroy all weapon actors when owner is destroyed
    (bind _weapon (Variables|/Game/AbilitySystem/Equipment/BP_EquipmentSlot.BP_EquipmentSlot_C|GetWeapon _array_element)
      (:then
        (Actor|DestroyActor _weapon))
      (:else))))

(fn Initialize
  (Utilities|FlowControl|Sequence
    (:then_0
      (for _array_element (Variables|Settings|GetEquipmentSlots) ; create slots
        (bind _returnvalue (Game|ConstructObjectfromClass (Components|GetOwner) "/Game/AbilitySystem/Equipment/BP_EquipmentSlot.BP_EquipmentSlot_C" _array_element))
        (Utilities|Array|Add (Variables|Don'tTouch|GetSlots) _returnvalue)))
    (:then_1
      (EquipmentManager|SwitchWeaponMode (Variables|Settings|GetDefaultWeaponMode)))))

(fn GetSlots
  (params (Type :type E_Equipment%20Enum :default "NewEnumerator11"))
  (for _array_element (Variables|Don'tTouch|GetSlots)
    (if (Utilities|Array|ContainsItem (.types (Variables|/Game/AbilitySystem/Equipment/BP_EquipmentSlot.BP_EquipmentSlot_C|GetSlotData _array_element)) Type) ; slot can be suitable for a few types (Sword, Axe etc)
      (Utilities|Array|Add (LocalVariables|GetlocalSlots) _array_element)))
  (return (LocalVariables|GetlocalSlots)))

(fn TryAddWeapontoSlot
  (params (Item :type S%20Item%20Data%20Structure))
  (LocalVariables|SetlocalSlot (Utilities|Array|Get(acopy) (EquipmentManager|GetSlots (.equipment Item))))
  (Utilities|FlowControl|Sequence
    (:then_0
      (if (Default|HasItem (LocalVariables|GetlocalSlot))
        (bind _out (EquipmentManager|TryRemoveWeaponfromSlot (LocalVariables|GetlocalSlot)))
        (if (not _out)
          (return false))))
    (:then_1
      (bind _returnvalue (Game|SpawnActorfromClass (.weapon Item) (Math|Transform|MakeTransform "0, 0, 0" "0, 0, 0" "1.000000,1.000000,1.000000") "Undefined" "SelectDefaultAtRuntime" (Components|GetOwner) 0))
      (Default|UpdateSlot (LocalVariables|GetlocalSlot) Item _returnvalue))
    (:then_2
      (if (Variables|/Game/AbilitySystem/Equipment/BP_EquipmentSlot.BP_EquipmentSlot_C|GetIsActive (LocalVariables|GetlocalSlot))
        (EquipmentManager|ActivateWeaponSlot (Utilities|Array|FindItem (Variables|Don'tTouch|GetSlots) (LocalVariables|GetlocalSlot)))
        (return true)
        (else
          (Transformation|AttachComponentToComponent (Variables|/Game/AbilitySystem/Equipment/BP_EquipmentSlot.BP_EquipmentSlot_C|GetWeapon (LocalVariables|GetlocalSlot)) (Variables|/Script/Engine.Character|GetMesh (.AsCharacter (Utilities|Casting|CastToCharacter (Components|GetOwner)))) (Variables|/Game/AbilitySystem/Equipment/Weapon/BP_Weapon.BP_Weapon_C|GetInactiveSocket (Variables|/Game/AbilitySystem/Equipment/BP_EquipmentSlot.BP_EquipmentSlot_C|GetWeapon (LocalVariables|GetlocalSlot))) "KeepRelative" "KeepRelative" "KeepRelative" true) ; attach weapon to inactive socket
          (return true))))))

(fn TryRemoveWeaponfromSlot
  (params (Slot :type BP%20Equipment%20Slot%20Object%20Reference))
  (Default|OnDeactivated (Variables|/Game/AbilitySystem/Equipment/BP_EquipmentSlot.BP_EquipmentSlot_C|GetWeapon (LocalVariables|GetlocalSlot)))
  (Actor|DestroyActor (Variables|/Game/AbilitySystem/Equipment/BP_EquipmentSlot.BP_EquipmentSlot_C|GetWeapon (LocalVariables|GetlocalSlot)))
  (Default|UpdateSlot (LocalVariables|GetlocalSlot))
  (return true))

(fn SwitchWeaponMode
  (params (Mode :type E_WeaponMode%20Enum :default "NewEnumerator0"))
  (if (Utilities|Enum|NotEqual(Enum) (Variables|Don'tTouch|GetCurrentWeaponMode) Mode)
    (if (Utilities|Enum|Equal(Enum) Mode "NewEnumerator0")
      (for _array_element (.slotindices (.Value (Utilities|Map|Find (Variables|Settings|GetWeaponModes) (Variables|Don'tTouch|GetCurrentWeaponMode)))) :!label _label ; deactivate all active slots
        (EquipmentManager|DeactivateWeaponSlot _array_element))
      (Variables|Don'tTouch|SetCurrentWeaponMode "NewEnumerator0")
      (else
        (Utilities|FlowControl|Sequence
          (:then_0
            (goto _label))
          (:then_1
            (Variables|Don'tTouch|SetCurrentWeaponMode Mode)
            (for _array_element_2 (.slotindices (.Value (Utilities|Map|Find (Variables|Settings|GetWeaponModes) (Variables|Don'tTouch|GetCurrentWeaponMode))))
              (EquipmentManager|ActivateWeaponSlot _array_element_2))))))))

(fn ActivateWeaponSlot
  (params (SlotIndex :type Integer))
  (LocalVariables|SetlocalSlot (Utilities|Array|Get(acopy) (Variables|Don'tTouch|GetSlots) SlotIndex))
  (Default|ChangeActiveState (LocalVariables|GetlocalSlot) true)
  (if (Default|HasItem (LocalVariables|GetlocalSlot))
    (Transformation|AttachComponentToComponent (Variables|/Game/AbilitySystem/Equipment/BP_EquipmentSlot.BP_EquipmentSlot_C|GetWeapon (LocalVariables|GetlocalSlot)) (Variables|/Script/Engine.Character|GetMesh (.AsCharacter (Utilities|Casting|CastToCharacter (Components|GetOwner)))) (Default|GetActiveSocket (Variables|/Game/AbilitySystem/Equipment/BP_EquipmentSlot.BP_EquipmentSlot_C|GetWeapon (LocalVariables|GetlocalSlot)) (.righthand (Variables|/Game/AbilitySystem/Equipment/BP_EquipmentSlot.BP_EquipmentSlot_C|GetSlotData (LocalVariables|GetlocalSlot)))) "KeepRelative" "KeepRelative" "KeepRelative" true) ; attach weapon to active socket
    (Default|OnActivated (Variables|/Game/AbilitySystem/Equipment/BP_EquipmentSlot.BP_EquipmentSlot_C|GetWeapon (LocalVariables|GetlocalSlot)))))

(fn DeactivateWeaponSlot
  (params (SlotIndex :type Integer))
  (LocalVariables|SetlocalSlot (Utilities|Array|Get(acopy) (Variables|Don'tTouch|GetSlots) SlotIndex))
  (Default|ChangeActiveState (LocalVariables|GetlocalSlot) false)
  (if (Default|HasItem (LocalVariables|GetlocalSlot))
    (Default|OnDeactivated (Variables|/Game/AbilitySystem/Equipment/BP_EquipmentSlot.BP_EquipmentSlot_C|GetWeapon (LocalVariables|GetlocalSlot)))
    (Transformation|AttachComponentToComponent (Variables|/Game/AbilitySystem/Equipment/BP_EquipmentSlot.BP_EquipmentSlot_C|GetWeapon (LocalVariables|GetlocalSlot)) (Variables|/Script/Engine.Character|GetMesh (.AsCharacter (Utilities|Casting|CastToCharacter (Components|GetOwner)))) (Variables|/Game/AbilitySystem/Equipment/Weapon/BP_Weapon.BP_Weapon_C|GetInactiveSocket (Variables|/Game/AbilitySystem/Equipment/BP_EquipmentSlot.BP_EquipmentSlot_C|GetWeapon (LocalVariables|GetlocalSlot))) "KeepRelative" "KeepRelative" "KeepRelative" true) ; attach weapon to inactive socket
  ))

(fn ThereIsWeaponwithThisTag
  (params (Weapon :type BP%20Weapon%20Object%20Reference) (Tag :type Gameplay%20Tag%20Structure))
  (for _array_element (Variables|Don'tTouch|GetSlots)
    (if (.weapon (Variables|/Game/AbilitySystem/Equipment/BP_EquipmentSlot.BP_EquipmentSlot_C|GetSlotData _array_element)) ; we need only weapon
      (Variables|/Game/AbilitySystem/Equipment/BP_EquipmentSlot.BP_EquipmentSlot_C|GetWeapon _array_element
        (:then
          (if (Variables|/Game/AbilitySystem/Equipment/BP_EquipmentSlot.BP_EquipmentSlot_C|GetIsActive _array_element)
            (if (!= (Variables|/Game/AbilitySystem/Equipment/BP_EquipmentSlot.BP_EquipmentSlot_C|GetWeapon _array_element) Weapon)
              (if (GameplayTags|HasTag (Variables|/Game/AbilitySystem/Equipment/Weapon/BP_Weapon.BP_Weapon_C|GetAppliedTags (Variables|/Game/AbilitySystem/Equipment/BP_EquipmentSlot.BP_EquipmentSlot_C|GetWeapon _array_element)) Tag true)
                (return true)))))
        (:else))))
  (return false))