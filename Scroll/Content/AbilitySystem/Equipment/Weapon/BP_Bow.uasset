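; Bow weapon equipment that puts its owning character into an aiming stance while active.
; Activation adds an aim widget task, applies the Goblin slingshot AnimInstance, plays a montage and switches rotation to controller-driven for strafing.
; It also spawns a CameraZoom actor for an offset aiming view.
; Deactivation ends the aim task, restores movement-oriented rotation and zooms out, but re-applies the same slingshot AnimInstance.
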(event EventOnDeactivated
  (bind _returnvalue (Components|GetOwner))
  (bind _ascharacter (Utilities|Casting|CastToCharacter _returnvalue))
  (bind _charactermovement (Variables|/Script/Engine.Character|GetCharacterMovement _ascharacter))
  (|CallParentFunction)
  (Utilities|FlowControl|Sequence
    (:then_0
      (bind _createaimbowtask (Variables|Default|GetCreateAimBowTask)
        (:then
          (Default|EndTask _createaimbowtask) ; remove Aim widget
        )
        (:else)))
    (:then_1
      (Default|ChangeAnimInstance (Variables|Default|GetOwnerAbilityManager) "/Game/Animations/Monster/Goblin/ABP_Goblin_Slingshot.ABP_Goblin_Slingshot_C")
      (Variables|/Script/Engine.CharacterMovementComponent|SetbOrientRotationToMovement _charactermovement true)
      (Variables|/Script/Engine.CharacterMovementComponent|SetbUseControllerDesiredRotation _charactermovement false))
    (:then_2
      (bind _camerazoomtask (Variables|Default|GetCameraZoomTask)
        (:then
          (Default|ZoomOut _camerazoomtask))
        (:else)))))

(event EventOnActivated
  (bind _returnvalue (Components|GetOwner))
  (bind _returnvalue_2 (Components|GetOwner))
  (bind _ascharacter (Utilities|Casting|CastToCharacter _returnvalue_2))
  (bind _charactermovement (Variables|/Script/Engine.Character|GetCharacterMovement _ascharacter))
  (|CallParentFunction)
  (bind _returnvalue_3 (AddComponent|AddAim (Components|GetOwner) 5e+03)) ; create Aim widget
  (Variables|Default|SetCreateAimBowTask _returnvalue_3)
  (Default|ChangeAnimInstance (Variables|Default|GetOwnerAbilityManager) "/Game/Animations/Monster/Goblin/ABP_Goblin_Slingshot.ABP_Goblin_Slingshot_C")
  (Animation|Montage|PlayMontage (Variables|/Script/Engine.Character|GetMesh (.AsCharacter (Utilities|Casting|CastToCharacter (Components|GetOwner)))) "/Game/Animations/Monster/Goblin/Animations/AdvancedAsset/BB_Sling_Down_Montage.BB_Sling_Down_Montage"
    (:then
      (Variables|/Script/Engine.CharacterMovementComponent|SetbOrientRotationToMovement _charactermovement false) ; id order to correctly implement BS_Archer we don't need to rotate character toward the velocity
      (Variables|/Script/Engine.CharacterMovementComponent|SetbUseControllerDesiredRotation _charactermovement true)
      (bind _returnvalue_4 (Game|SpawnActorfromClass "/Game/AbilitySystem/Tasks/CameraZoom.CameraZoom_C" (Transformation|GetActorTransform _returnvalue) "Undefined" "OverrideRootScale" _returnvalue 3.3 3.3 4e+02 "0.000000,60.000000,70.000000" 0)) ; ZoomIn/ZoomOut camera
      (Variables|Default|SetCameraZoomTask _returnvalue_4))))

(fn ConstructionScript)