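; AI bow weapon equipment that switches its owning character into a slingshot-based ranged stance.
; On activation it sets the goblin slingshot anim instance through the ability manager, plays the raise montage and disables OrientRotationToMovement to support the BS_Archer blendspace.
; Deactivation restores movement-oriented rotation but applies the same slingshot anim instance rather than a different one.
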(event EventOnActivated
  (|CallParentFunction)
  (Default|ChangeAnimInstance (Variables|Default|GetOwnerAbilityManager) "/Game/Animations/Monster/Goblin/ABP_Goblin_Slingshot.ABP_Goblin_Slingshot_C")
  (Animation|Montage|PlayMontage (Variables|/Script/Engine.Character|GetMesh (.AsCharacter (Utilities|Casting|CastToCharacter (Components|GetOwner)))) "/Game/Animations/Monster/Goblin/Animations/AdvancedAsset/BB_Sling_Up.BB_Sling_Up"
    (:then
      (Variables|/Script/Engine.CharacterMovementComponent|SetbOrientRotationToMovement (Variables|/Script/Engine.Character|GetCharacterMovement (.AsCharacter (Utilities|Casting|CastToCharacter (Components|GetOwner)))) false) ; id order to correctly implement BS_Archer we don't need to rotate character toward the velocity
    )))

(event EventOnDeactivated
  (|CallParentFunction)
  (Default|ChangeAnimInstance (Variables|Default|GetOwnerAbilityManager) "/Game/Animations/Monster/Goblin/ABP_Goblin_Slingshot.ABP_Goblin_Slingshot_C")
  (Variables|/Script/Engine.CharacterMovementComponent|SetbOrientRotationToMovement (Variables|/Script/Engine.Character|GetCharacterMovement (.AsCharacter (Utilities|Casting|CastToCharacter (Components|GetOwner)))) true))

(fn ConstructionScript)