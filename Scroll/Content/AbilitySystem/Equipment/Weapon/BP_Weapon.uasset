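; Base weapon Blueprint that grants gameplay tags to its owner while active and provides the right- or left-hand socket for its active state.
; On begin play it caches the owner's ability and equipment managers through message calls, then applies its tags on activation.
; On deactivation it removes them only if the equipment manager finds no weapon sharing its ActiveWeapon child tag, so dual-wielded swords keep their tags.
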(event Custom|OnActivated
  (Default|ApplyTags (Variables|Default|GetOwnerAbilityManager) (Variables|WeaponSettings|GetAppliedTags)))

(event Custom|OnDeactivated
  (if (not (Default|ThereIsWeaponwithThisTag (Variables|Default|GetEquipmentManager) self (CallFunction|GetTagbyParent (Variables|WeaponSettings|GetAppliedTags) "(TagName=\"ActiveWeapon\")"))) ; if 2 sword are equipped, we don't need to remove tags when we unequip first sword
    (Default|RemoveTags (Variables|Default|GetOwnerAbilityManager) (Variables|WeaponSettings|GetAppliedTags))))

(event EventBeginPlay
  (bind _manager (Class|BIAbilitySystemActor|GetAbilityManager(Message) (Components|GetOwner)))
  (Variables|Default|SetOwnerAbilityManager _manager)
  (bind _manager_2 (Class|BIAbilityEquipmentActor|GetEquipmentManagerA(Message) (Components|GetOwner)))
  (Variables|Default|SetEquipmentManager _manager_2))

(fn ConstructionScript)

(fn GetActiveSocket
  (params (RightHand :type Boolean))
  (return (select RightHand (Variables|WeaponSettings|GetRightActiveSocket) (Variables|WeaponSettings|GetLeftActiveSocket))))