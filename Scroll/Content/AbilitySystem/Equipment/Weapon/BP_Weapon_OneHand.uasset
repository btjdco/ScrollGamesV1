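; One-handed weapon Blueprint in the ability system's equipment set, extending a parent weapon class.
; On activation it runs the parent logic, switches the owner's anim instance to the Goblin Warrior AnimBP through the ability manager, and plays a take montage on the owning Character's mesh.
; Deactivation runs the parent logic and sets that same AnimBP again, with no montage.
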(event EventOnDeactivated
  (|CallParentFunction)
  (Default|ChangeAnimInstance (Variables|Default|GetOwnerAbilityManager) "/Game/Animations/Monster/Goblin/ABP_Goblin_Warrior.ABP_Goblin_Warrior_C"))

(event EventOnActivated
  (|CallParentFunction)
  (Default|ChangeAnimInstance (Variables|Default|GetOwnerAbilityManager) "/Game/Animations/Monster/Goblin/ABP_Goblin_Warrior.ABP_Goblin_Warrior_C")
  (Animation|Montage|PlayMontage (Variables|/Script/Engine.Character|GetMesh (.AsCharacter (Utilities|Casting|CastToCharacter (Components|GetOwner)))) "/Game/Animations/Monster/Goblin/Animations/AdvancedAsset/BB_Goblin_Take.BB_Goblin_Take"))

(fn ConstructionScript
  (|CallParentFunction))