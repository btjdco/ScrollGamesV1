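; Base AI character for the ability system, supplying start attributes, tags, effects and abilities from AIData and showing interaction widgets.
; Incoming damage is absorbed by Shield on blockable frontal hits, with any remainder going to Health, then displayed in world with a temporary attribute bar.
; Health changes toggle a regeneration effect.
; At zero Health, it stops AI logic, applies the Dead tag, plays a death animation and destroys itself after a delay.
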(event EventBeginPlay)

(event EventHideInteractionInfoA
  (Components|DestroyComponent (Variables|Default|GetInteractionWidget)))

(event EventShowInteractionInfoA
  (bind _returnvalue (AddComponent|AddWidgetComponent false (Math|Transform|MakeTransform "0, 0,100.000000" "0, 0, 0" "1.000000,1.000000,1.000000"))) ; select the node\nwidget is set in details panel
  (Variables|Default|SetInteractionWidget _returnvalue))

(event EventAnyDamage
  (params (DamageData :type S%20Damage%20Data%20Structure))
  (bind _outdamagedata (CallFunction|DistributeDamage DamageData))
  (CallFunction|ShowDamageDatainWorld _outdamagedata) ; see parent class
  (bind _health (Variables|Default|GetHealth)
    (:then
      (if (== (Variables|/Game/AbilitySystem/BP_Attribute.BP_Attribute_C|GetCurrentValue _health) 0.0) ; Health = 0
        (CallFunction|Death)
        (else
          (Variables|Default|GetAttributeBar
            (:then
              _)
            (:else
              (bind _returnvalue (AddComponent|AddWCAttributeBarAI false (Math|Transform|MakeTransform "0, 0,100.000000" "0, 0, 0" "1.000000,1.000000,1.000000")))
              (Variables|Default|SetAttributeBar _returnvalue)))
          (Utilities|FlowControl|RetriggerableDelay 5.0)
          (bind _attributebar (Variables|Default|GetAttributeBar)
            (:then
              (Components|DestroyComponent _attributebar))
            (:else)))))
    (:else)))

(event EventDeath
  (AI|Logic|StopLogic (Variables|/Script/AIModule.AIController|GetBrainComponent (AI|GetAIController self)) "")
  (Default|ApplyTags (Variables|Default|GetAbilityManager) "(GameplayTags=((TagName=\"State.Dead\")))") ; turn off all regeneration\nalso Player can't attack, and AI can't move
  (Components|Animation|PlayAnimation (Variables|Character|GetMesh) (Variables|Default|GetDeathAnimation) false) ; i think we don't need to handle this via Animation Blueprint (state machine)\nwe can just play this anim one time
  (Collision|SetCollisionResponsetoChannel (Variables|Default|GetCapsuleComponent) "ECC_Pawn" "ECR_Ignore")
  (Default|RemoveAllAppliedEffects (Variables|Default|GetAbilityManager))
  (bind _attributebar (Variables|Default|GetAttributeBar)
    (:then
      (Components|DestroyComponent _attributebar))
    (:else
      _))
  (Utilities|FlowControl|Delay 2e+01)
  (Actor|DestroyActor))

(event EventInteractionA
  (AddComponent|AddWCGreeting true (Transformation|GetActorTransform)))

(event EventInitializeAbilityManager
  (Default|Initialize (Variables|Default|GetAbilityManager))
  (|AbilityManager))

(fn ConstructionScript
  (|CallParentFunction))

(fn GetStartData
  (bind _aidata (Variables|Default|GetAIData))
  (return (Variables|/Game/AbilitySystem/Global/AI/PDA_AIData.PDA_AIData_C|GetAttributes _aidata) (Variables|/Game/AbilitySystem/Global/AI/PDA_AIData.PDA_AIData_C|GetAppliedTags _aidata) (Variables|/Game/AbilitySystem/Global/AI/PDA_AIData.PDA_AIData_C|GetEffects _aidata) (Variables|/Game/AbilitySystem/Global/AI/PDA_AIData.PDA_AIData_C|GetAbilities _aidata) (Variables|/Game/AbilitySystem/Global/AI/PDA_AIData.PDA_AIData_C|GetExecutions _aidata) (Variables|Default|GetStartLevel) (Variables|/Game/AbilitySystem/Global/AI/PDA_AIData.PDA_AIData_C|GetMaxLevel _aidata) "" ""))

(fn GetInteractionDistance
  (return 2.5e+02))

(fn DistributeDamage
  (params (DamageData :type S%20Damage%20Data%20Structure))
  (LocalVariables|SetlocalDamage (.damage DamageData))
  (Utilities|FlowControl|Sequence
    (:then_0
      (Variables|Default|GetShield
        (:then
          (if (GameplayTags|HasTag (Variables|/Game/AbilitySystem/AC_AbilityManager.AC_AbilityManager_C|GetGameplayTags (Variables|Default|GetAbilityManager)) (Variables|/Game/AbilitySystem/AC_AbilityManager.AC_AbilityManager_C|GetFrontalBlockTag (Variables|Default|GetAbilityManager)) true) ; Frontal Block
            (if (GameplayTags|HasTag (Utilities|Struct|BreakS_DamageData DamageData) "(TagName=\"Damage.CanBeBlocked\")" true)
              (if (CallFunction|IsImpactfromFront self (Utilities|Struct|BreakS_DamageData DamageData))
                (GameplayTags|AddGameplayTag (Utilities|Struct|BreakS_DamageData DamageData) "(TagName=\"Damage.Blocked\")" :!class /Script/GameplayTags.BlueprintGameplayTagLibrary)
                (if (>= (Variables|/Game/AbilitySystem/BP_Attribute.BP_Attribute_C|GetCurrentValue (Variables|Default|GetShield)) (LocalVariables|GetlocalDamage))
                  (Default|ModifyAttribute (Variables|Default|GetAbilityManager) "NewEnumerator24" "NewEnumerator1" "NewEnumerator1" (LocalVariables|GetlocalDamage))
                  (return DamageData)
                  (else
                    (LocalVariables|SetlocalDamage (- (LocalVariables|GetlocalDamage) (Variables|/Game/AbilitySystem/BP_Attribute.BP_Attribute_C|GetCurrentValue (Variables|Default|GetShield))))
                    (Default|ModifyAttribute (Variables|Default|GetAbilityManager) "NewEnumerator24" "NewEnumerator1" "NewEnumerator1" (Variables|/Game/AbilitySystem/BP_Attribute.BP_Attribute_C|GetCurrentValue (Variables|Default|GetShield)))))))))
        (:else)))
    (:then_1
      (Default|ModifyAttribute (Variables|Default|GetAbilityManager) "NewEnumerator13" "NewEnumerator1" "NewEnumerator1" (LocalVariables|GetlocalDamage))
      (return DamageData))))

(event Custom|HandleHealthRegeneration
  (bind _health (Variables|Default|GetHealth))
  (if (< (Variables|/Game/AbilitySystem/BP_Attribute.BP_Attribute_C|GetCurrentValue (Variables|Default|GetHealth)) (|(RealValue-(RealValue*Blocked)) (Variables|/Game/AbilitySystem/BP_Attribute.BP_Attribute_C|GetRealValue _health) (Variables|/Game/AbilitySystem/BP_Attribute.BP_Attribute_C|GetBlockedValue _health)))
    (bind _aeffect (Default|GetEffect (Variables|Default|GetAbilityManager) "/Game/AbilitySystem/Effects/HealthRegeneration.HealthRegeneration_C"))
    (Utilities|IsValid _aeffect
      (:Is%20Not%20Valid
        (Default|ApplyEffect (Variables|Default|GetAbilityManager) (Utilities|Struct|MakeS_EffectData "/Game/AbilitySystem/Effects/MonsterHealthRegeneration.MonsterHealthRegeneration_C" 1 0 false "(Tick_17_40755E2C4DCAD94CF3DBA2AECC805C15=(Source_10_0C1CA74C4C120C42C1F857BD53F0A76F=NewEnumerator0,Value_5_90E89AB144D6F3B57A2FB59966A03498=0.000000,CurveTable_11_2B4B079B4C7ECA70D04E3F947A964B45=(CurveTable=None,RowName=\"\")),ChanceToApply_19_3C8E08B246FF3BA8A2CDA8A8D9F764C6=(Source_10_0C1CA74C4C120C42C1F857BD53F0A76F=NewEnumerator0,Value_5_90E89AB144D6F3B57A2FB59966A03498=0.000000,CurveTable_11_2B4B079B4C7ECA70D04E3F947A964B45=(CurveTable=None,RowName=\"\")),Duration_29_7F8704364211410D0930AD8AB240975B=(Source_10_0C1CA74C4C120C42C1F857BD53F0A76F=NewEnumerator0,Value_5_90E89AB144D6F3B57A2FB59966A03498=0.000000,CurveTable_11_2B4B079B4C7ECA70D04E3F947A964B45=(CurveTable=None,RowName=\"\")),DurationPolicy_32_683FC34B46CBA1C769699589F12C9837=NewEnumerator1,ExpirationPolicy_36_54D3E72548F23CD877ABE988E2FC308D=NewEnumerator0)" false "0.000000,0.000000,0.000000")) ; Apply Health Regeneration Effect
      ))
    (else
      (Default|RemoveEffectbyClass (Variables|Default|GetAbilityManager) "/Game/AbilitySystem/Effects/MonsterHealthRegeneration.MonsterHealthRegeneration_C") ; Remove Health Regeneration Effect
    )))