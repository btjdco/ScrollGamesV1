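; Defensive tower AI that attacks the player within its sphere radius, built on an AbilityManager component for attributes, tags and abilities.
; Player overlap starts a looping timer and Tower_Attack, skipped if the player is dead; leaving cancels both.
; Damage reduces health, shows damage data and briefly reveals the health bar; zero health tags it destroyed, rotates the mesh and stops attacks.
; Interaction levels up the tower through the AbilityManager.
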(event OnComponentBeginOverlap(Sphere)
  (params (OverlappedComponent :type Primitive%20Component%20Object%20Reference) (OtherActor :type Actor%20Object%20Reference) (OtherComp :type Primitive%20Component%20Object%20Reference) (OtherBodyIndex :type Integer) (bFromSweep :type Boolean) (SweepResult :type Hit%20Result%20Structure%20%28by%20ref%29))
  (if (and (== OtherActor (Game|GetPlayerCharacter 0)) (not (GameplayTags|HasTag (Variables|/Game/AbilitySystem/AC_AbilityManager.AC_AbilityManager_C|GetGameplayTags (Variables|Default|GetAbilityManager)) "(TagName=\"Tower.Destroyed\")" true)))
    (bind _returnvalue (Utilities|Time|SetTimerbyEvent (EventDispatchers|CreateEvent :!event Custom|Attack) 1.0 true)) ; ability and timer are activated when player overlaps Tower's area
    (Variables|Default|SetAttackTimer _returnvalue)
    (CallFunction|Attack)))

(event OnComponentEndOverlap(Sphere)
  (params (OverlappedComponent :type Primitive%20Component%20Object%20Reference) (OtherActor :type Actor%20Object%20Reference) (OtherComp :type Primitive%20Component%20Object%20Reference) (OtherBodyIndex :type Integer))
  (if (== OtherActor (Game|GetPlayerCharacter 0))
    (CallFunction|CancelAttack)))

(event Custom|OnDestroy
  (Default|ApplyTags (Variables|Default|GetAbilityManager) "(GameplayTags=((TagName=\"Tower.Destroyed\")))")
  (Transformation|SetRelativeRotation (Variables|Default|GetStaticMesh) (Variables|Default|GetDestroyedRotation) false false)
  (CallFunction|CancelAttack))

(event Custom|Attack
  (bind _manager (Class|BIAbilitySystemActor|GetAbilityManager(Message) (Game|GetPlayerCharacter 0)))
  (if (not (GameplayTags|HasTag (Variables|/Game/AbilitySystem/AC_AbilityManager.AC_AbilityManager_C|GetGameplayTags _manager) "(TagName=\"State.Dead\")" true))
    (Default|TryActivateAbility (Variables|Default|GetAbilityManager) "/Game/AbilitySystem/Abilities/Tower_Attack.Tower_Attack_C")))

(event Custom|CancelAttack
  (Utilities|Time|ClearandInvalidateTimerbyHandle (Variables|Default|GetAttackTimer)) ; Diactivate timer when player leaves Tower's area
  (Default|CancelAbilitybyClass (Variables|Default|GetAbilityManager) "/Game/AbilitySystem/Abilities/Tower_Attack.Tower_Attack_C"))

(event EventShowDatainWorld
  (bind _returnvalue (Actor|GetComponentbyClass "/Game/AbilitySystem/GUI/AbilitySystem/WC_TargetData.WC_TargetData_C"))
  (Utilities|IsValid _returnvalue
    (:Is%20Valid
      (Components|DestroyComponent _returnvalue))
    (:Is%20Not%20Valid
      (AddComponent|AddWCTargetData false (Math|Transform|MakeTransform "0, 0,250.000000" "0, 0, 0" "1.000000,1.000000,1.000000")))))

(event EventShowDamageDatainWorld
  (params (DamageData :type S%20Damage%20Data%20Structure))
  (AddComponent|AddWCDamage true (Transformation|GetActorTransform) DamageData))

(event EventInteractionA
  (Default|AILevelUp (Variables|Default|GetAbilityManager) (+ (Variables|/Game/AbilitySystem/AC_AbilityManager.AC_AbilityManager_C|GetCurrentLevel (Variables|Default|GetAbilityManager)) 1)))

(event EventAnyDamage
  (params (DamageData :type S%20Damage%20Data%20Structure))
  (Default|ModifyAttribute (Variables|Default|GetAbilityManager) "NewEnumerator13" "NewEnumerator1" "NewEnumerator1" (.Damage (Utilities|Struct|BreakS_DamageData DamageData)))
  (CallFunction|ShowDamageDatainWorld DamageData)
  (if (== (Variables|/Game/AbilitySystem/BP_Attribute.BP_Attribute_C|GetCurrentValue (Default|GetAttribute (Variables|Default|GetAbilityManager) "NewEnumerator13")) 0.0) ; Health = 0
    (CallFunction|OnDestroy)
    (else
      (Rendering|SetVisibility (Variables|Default|GetHealthBar) true false)
      (Utilities|FlowControl|RetriggerableDelay 5.0)))
  (Rendering|SetVisibility (Variables|Default|GetHealthBar) false false))

(event EventBeginPlay
  (Default|Initialize (Variables|Default|GetAbilityManager))
  (Default|Initialize (.AsWBP%20Attribute%20Bar%20AI (Utilities|Casting|CastToWBP_AttributeBar_AI (UserInterface|GetUserWidgetObject (Variables|Default|GetHealthBar)))) self) ; bind health bar with health Attribute
)

(fn ConstructionScript
  (Components|Sphere|SetSphereRadius (Variables|Default|GetSphere) (Variables|Settings|GetSphereRadius) true))

(fn CanAttackA
  (return (Default|CanbeAttacked (Variables|Default|GetAbilityManager))))

(fn CanInteractA
  (return (Default|CanbeInteracted (Variables|Default|GetAbilityManager))))

(fn GetAbilityManager
  (return (Variables|Default|GetAbilityManager)))

(fn GetInteractionDistance
  (return 3e+02))

(fn GetStartData
  (return (Variables|Settings|GetAttributes) (Variables|Settings|GetAppliedTags) 0 (Variables|Settings|GetAbilities) (Variables|Settings|GetStartExecutions) (Variables|Settings|GetStartLevel) (Variables|Settings|GetMaxLevel) "" ""))