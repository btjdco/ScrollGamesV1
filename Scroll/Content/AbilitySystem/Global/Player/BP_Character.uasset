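; BP_Character is a character Blueprint in the ability system that exposes combat, interaction and debug-display hooks.
; Attack and interaction checks defer to its AbilityManager, and getters expose that manager and the AbilityEquipmentManager.
; ShowDatainWorld toggles a target-data widget component above the character, while ShowDamageDatainWorld spawns a damage widget component at its transform.
; Death and DistributeDamage are empty, and the distance and level getters return zero.
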(event Custom|Death)

(event EventShowDatainWorld
  (bind _returnvalue (Actor|GetComponentbyClass "/Game/AbilitySystem/GUI/AbilitySystem/WC_TargetData.WC_TargetData_C"))
  (Utilities|IsValid _returnvalue
    (:Is%20Valid
      (Components|DestroyComponent _returnvalue))
    (:Is%20Not%20Valid
      (AddComponent|AddWCTargetData false (Math|Transform|MakeTransform "0, 0,250.000000" "0, 0, 0" "1.000000,1.000000,1.000000")))))

(event EventShowDamageDatainWorld
  (params (DamageData :type S%20Damage%20Data%20Structure))
  (AddComponent|AddWCDamage true (Transformation|GetActorTransform) DamageData))

(fn ConstructionScript)

(fn DistributeDamage
  (params (DamageData :type S%20Damage%20Data%20Structure))
  (return ""))

(fn CanAttackA
  (return (Default|CanbeAttacked (Variables|Default|GetAbilityManager))))

(fn CanInteractA
  (return (Default|CanbeInteracted (Variables|Default|GetAbilityManager))))

(fn GetAbilityManager
  (return (Variables|Default|GetAbilityManager)))

(fn GetEquipmentManagerA
  (return (Variables|Default|GetAbilityEquipmentManager)))

(fn GetInteractionDistance
  (return 0.0))

(fn GetStartData
  (return 0 "" 0 0 0 0 0 "" ""))