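; Player character Blueprint that ties AbilityManager attributes to damage, death and respawn.
; Attribute modify events toggle regeneration effects for Health, Mana, Energy and Shield.
; Damage passes through temporary shield, frontal block and Mana Shield before Health, while fall damage, scaled by drop from timer-sampled peak height, hits Health directly.
; Zero Health applies a dead tag and plays a death animation, then respawns at a PlayerStart with attributes restored.
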(event Custom|Respawn
  (bind _returnvalue (Actor|GetActorOfClass "/Script/Engine.PlayerStart"))
  (Transformation|SetActorLocation (Transformation|GetActorLocation _returnvalue) false false)
  (Components|Animation|SetAnimationMode (Variables|Character|GetMesh) "AnimationBlueprint") ; since we played 'death' animation, our skeletal mesh is in 'use cusom' mode\nin order to use Animation Blueprint, we need set this mode manually
  (Default|RemoveTags (Variables|Default|GetAbilityManager) "(GameplayTags=((TagName=\"State.Dead\")))")
  (bind _returnvalue_2 (Game|ConstructObjectfromClass "/Game/AbilitySystem/Executions/RestoreAttributes.RestoreAttributes_C" self 0 0 0)) ; restore Health, Mana, Shield, Energy
  (Default|Execute _returnvalue_2))

(event Custom|CheckMaxHeight
  ;[1 1 1] Fall Damage
  (if (> (.z (Transformation|GetActorLocation)) (Variables|Default|GetFallHeight))
    (Variables|Default|SetFallHeight (.z (Transformation|GetActorLocation))) ; here we will get max Z position
  ))

(event EventAnyDamage
  (params (DamageData :type S%20Damage%20Data%20Structure))
  (bind _outdamagedata (CallFunction|DistributeDamage DamageData))
  (Default|CallOnReceiveDamage (Variables|Default|GetAbilityManager) _outdamagedata)
  (CallFunction|ShowDamageDatainWorld _outdamagedata) ; see parent class
  (if (== (Variables|/Game/AbilitySystem/BP_Attribute.BP_Attribute_C|GetCurrentValue (Variables|Default|GetHealth)) 0.0)
    (CallFunction|Death)))

(event EventOnMovementModeChanged
  (params (PrevMovementMode :type EMovementMode%20Enum :default "MOVE_None") (NewMovementMode :type EMovementMode%20Enum :default "MOVE_None") (PrevCustomMode :type Byte :default 0) (NewCustomMode :type Byte :default 0))
  ;[1 1 1] Fall Damage
  (if (Utilities|Enum|Equal(Enum) NewMovementMode "MOVE_Falling")
    (bind _out (Default|IsCastingAbility (Variables|Default|GetAbilityManager))) ; character can use abilities with jumping\nlet's by design we don't react on a such cases
    (if (not _out)
      (Variables|Default|SetFallHeight (.z (Transformation|GetActorLocation))) ; save start Z position
      (bind _returnvalue (Utilities|Time|SetTimerbyEvent (delegate Custom|CheckMaxHeight) 0.1 true))
      (Variables|Default|SetFallTimer _returnvalue))))

(event EventOnLanded
  (params (Hit :type Hit%20Result%20Structure%20%28by%20ref%29))
  (bind _returnvalue (Transformation|GetActorLocation))
  (bind _self self)
  ;[1 1 1] Fall Damage
  (if (Utilities|Time|IsTimerActivebyHandle (Variables|Default|GetFallTimer))
    (Utilities|Time|ClearandInvalidateTimerbyHandle (Variables|Default|GetFallTimer))
    (Variables|Default|SetFallDistance (Math|Vector|Distance(Vector) (Transformation|GetActorLocation) (Math|Vector|MakeVector (.x _returnvalue) (.y _returnvalue) (Variables|Default|GetFallHeight))))
    (if (>= (Variables|Default|GetFallDistance) 5e+02) ; don't react on small jump
      (Class|BIAbilitySystemActor|AnyDamage(Message) self (Utilities|Struct|MakeS_DamageData (Utilities|Struct|MakeGameplayTagContainer (Utilities|Array|MakeArray (Variables|/Game/AbilitySystem/AC_AbilityManager.AC_AbilityManager_C|GetFallDamageTag (Variables|Default|GetAbilityManager)))) (* (Variables|/Game/AbilitySystem/BP_Attribute.BP_Attribute_C|GetRealValue (Default|GetAttribute (Variables|Default|GetAbilityManager) "NewEnumerator13")) (Math|Float|MapRangeClamped (Variables|Default|GetFallDistance) 5e+02 2e+03 0.1 1.0)) _self _self "0.000000,0.000000,0.000000")))))

(event EventDeath
  (Utilities|FlowControl|DoOnce false :!label _label
    (:Completed
      (Default|ApplyTags (Variables|Default|GetAbilityManager) "(GameplayTags=((TagName=\"State.Dead\")))") ; turn off all regeneration\nalso AI can't attack and player can't move
      (Components|Animation|PlayAnimation (Variables|Character|GetMesh) (Variables|Default|GetDeathAnimation) false) ; i think we don't need to handle this via Animation Blueprint (state machine)\nwe can just play this anim one time
      (Default|CancelCurrentlyCastedAbility (Variables|Default|GetAbilityManager))
      (Utilities|FlowControl|Delay 5.0)
      (CallFunction|Respawn)
      (goto _label Reset))))

(event EventInitializeAbilityManager
  (Default|Initialize (Variables|Default|GetAbilityManager))
  (|AbilityManager))

(fn ConstructionScript
  (|CallParentFunction))

(fn DistributeDamage
  (params (DamageData :type S%20Damage%20Data%20Structure))
  (LocalVariables|SetlocalDamage (.damage DamageData))
  (if (GameplayTags|HasTag (.tags DamageData) (Variables|/Game/AbilitySystem/AC_AbilityManager.AC_AbilityManager_C|GetFallDamageTag (Variables|Default|GetAbilityManager)) true)
    (Default|ModifyAttribute (Variables|Default|GetAbilityManager) "NewEnumerator13" "NewEnumerator1" "NewEnumerator1" (LocalVariables|GetlocalDamage))
    (return DamageData)
    (else
      (Utilities|FlowControl|Sequence
        (:then_0
          ;[1 1 1] Temporary Shield Effect that absorbs damage
          (Variables|Default|GetShieldAbility ; if valid, ability is activated and we can absorb damage
            (:then
              _)
            (:else
              (bind _aability (Default|GetAbilitybyClass (Variables|Default|GetAbilityManager) "/Game/AbilitySystem/Abilities/Overall_TemporaryShield.Overall_TemporaryShield_C"))
              (Variables|Default|SetShieldAbility _aability)
              (Variables|Default|GetShieldAbility
                (:then
                  _)
                (:else))))
          (bind _newdamage (Default|AbsorbDamage (.AsOverall%20Temporary%20Shield (Utilities|Casting|CastToOverall_TemporaryShield (Variables|Default|GetShieldAbility))) (LocalVariables|GetlocalDamage)))
          (LocalVariables|SetlocalDamage _newdamage)
          (Default|CheckStatus (.AsOverall%20Temporary%20Shield (Utilities|Casting|CastToOverall_TemporaryShield (Variables|Default|GetShieldAbility)))))
        (:then_1
          (Variables|Default|GetShield
            (:then
              (if (GameplayTags|HasTag (Variables|/Game/AbilitySystem/AC_AbilityManager.AC_AbilityManager_C|GetGameplayTags (Variables|Default|GetAbilityManager)) (Variables|/Game/AbilitySystem/AC_AbilityManager.AC_AbilityManager_C|GetFrontalBlockTag (Variables|Default|GetAbilityManager)) true) ; Frontal Block
                (if (GameplayTags|HasTag (Utilities|Struct|BreakS_DamageData DamageData) "(TagName=\"Damage.CanBeBlocked\")" true)
                  (if (CallFunction|IsImpactfromFront self (Utilities|Struct|BreakS_DamageData DamageData))
                    (GameplayTags|AddGameplayTag (Utilities|Struct|BreakS_DamageData DamageData) "(TagName=\"Damage.Blocked\")" :!class /Script/GameplayTags.BlueprintGameplayTagLibrary)
                    (if (>= (Variables|/Game/AbilitySystem/BP_Attribute.BP_Attribute_C|GetCurrentValue (Variables|Default|GetShield)) (LocalVariables|GetlocalDamage))
                      (Default|ModifyAttribute (Variables|Default|GetAbilityManager) "NewEnumerator24" "NewEnumerator1" "NewEnumerator1" (LocalVariables|GetlocalDamage))
                      (return DamageData)
                      (else
                        (LocalVariables|SetlocalDamage (- (LocalVariables|GetlocalDamage) (Variables|/Game/AbilitySystem/BP_Attribute.BP_Attribute_C|GetCurrentValue (Variables|Default|GetShield))))
                        (Default|ModifyAttribute (Variables|Default|GetAbilityManager) "NewEnumerator24" "NewEnumerator1" "NewEnumerator1" (Variables|/Game/AbilitySystem/BP_Attribute.BP_Attribute_C|GetCurrentValue (Variables|Default|GetShield)))))))))
            (:else)))
        (:then_2
          ;[1 1 1] ManaShield effect
          (bind _aeffect (Default|GetEffect (Variables|Default|GetAbilityManager) "/Game/AbilitySystem/Effects/ManaShield.ManaShield_C"))
          (LocalVariables|SetlocalManaShieldEffect _aeffect)
          (LocalVariables|GetlocalManaShieldEffect
            (:then
              (bind _out (Class|BIEffect|GetSpecialValue(Message) (LocalVariables|GetlocalManaShieldEffect))) ; open Mana Shield effect class to see the function implementation
              (LocalVariables|SetlocalManaShieldCoefficient _out)
              (if (>= (Variables|/Game/AbilitySystem/BP_Attribute.BP_Attribute_C|GetCurrentValue (Variables|Default|GetMana)) (* (LocalVariables|GetlocalDamage) (LocalVariables|GetlocalManaShieldCoefficient)))
                (Default|ModifyAttribute (Variables|Default|GetAbilityManager) "NewEnumerator14" "NewEnumerator1" "NewEnumerator1" (* (LocalVariables|GetlocalDamage) (LocalVariables|GetlocalManaShieldCoefficient)))
                (LocalVariables|SetlocalDamage (- (LocalVariables|GetlocalDamage) (* (LocalVariables|GetlocalDamage) (LocalVariables|GetlocalManaShieldCoefficient))))
                (else
                  (LocalVariables|SetlocalDamage (- (LocalVariables|GetlocalDamage) (Variables|/Game/AbilitySystem/BP_Attribute.BP_Attribute_C|GetCurrentValue (Variables|Default|GetMana))))
                  (Default|ModifyAttribute (Variables|Default|GetAbilityManager) "NewEnumerator14" "NewEnumerator1" "NewEnumerator1" (Variables|/Game/AbilitySystem/BP_Attribute.BP_Attribute_C|GetCurrentValue (Variables|Default|GetMana))))))
            (:else)))
        (:then_3
          (Default|ModifyAttribute (Variables|Default|GetAbilityManager) "NewEnumerator13" "NewEnumerator1" "NewEnumerator1" (LocalVariables|GetlocalDamage) :!pinned true) ; Health
        )
        (:then_4
          (return DamageData))))))

(fn GetStartData
  (bind _startdata (Variables|Default|GetStartData))
  (return (Variables|/Game/AbilitySystem/Global/PDA_PlayerData.PDA_PlayerData_C|GetAttributes _startdata) (Variables|/Game/AbilitySystem/Global/PDA_PlayerData.PDA_PlayerData_C|GetAppliedTags _startdata) (Variables|/Game/AbilitySystem/Global/PDA_PlayerData.PDA_PlayerData_C|GetEffects _startdata) (Variables|/Game/AbilitySystem/Global/PDA_PlayerData.PDA_PlayerData_C|GetAbilities _startdata) (Variables|/Game/AbilitySystem/Global/PDA_PlayerData.PDA_PlayerData_C|GetExecutions _startdata) (Variables|/Game/AbilitySystem/Global/PDA_PlayerData.PDA_PlayerData_C|GetStartLevel _startdata) (Variables|/Game/AbilitySystem/Global/PDA_PlayerData.PDA_PlayerData_C|GetMaxLevel _startdata) (Variables|/Game/AbilitySystem/Global/PDA_PlayerData.PDA_PlayerData_C|GetBoostPointsReward _startdata) (Variables|/Game/AbilitySystem/Global/PDA_PlayerData.PDA_PlayerData_C|GetExpToLevelUp _startdata)))

(fn CanAttackA
  (return (Default|CanbeAttacked (Variables|Default|GetAbilityManager))))

(event Custom|HandleShieldRegeneration
  (bind _shield (Variables|Default|GetShield))
  (if (< (Variables|/Game/AbilitySystem/BP_Attribute.BP_Attribute_C|GetCurrentValue (Variables|Default|GetShield)) (|(RealValue-(RealValue*Blocked)) (Variables|/Game/AbilitySystem/BP_Attribute.BP_Attribute_C|GetRealValue _shield) (Variables|/Game/AbilitySystem/BP_Attribute.BP_Attribute_C|GetBlockedValue _shield)))
    (Default|ApplyEffect (Variables|Default|GetAbilityManager) (Utilities|Struct|MakeS_EffectData "/Game/AbilitySystem/Effects/ShieldRegeneration.ShieldRegeneration_C" 1 0 false "(Tick_17_40755E2C4DCAD94CF3DBA2AECC805C15=(Source_10_0C1CA74C4C120C42C1F857BD53F0A76F=NewEnumerator0,Value_5_90E89AB144D6F3B57A2FB59966A03498=0.000000,CurveTable_11_2B4B079B4C7ECA70D04E3F947A964B45=(CurveTable=None,RowName=\"\")),ChanceToApply_19_3C8E08B246FF3BA8A2CDA8A8D9F764C6=(Source_10_0C1CA74C4C120C42C1F857BD53F0A76F=NewEnumerator0,Value_5_90E89AB144D6F3B57A2FB59966A03498=0.000000,CurveTable_11_2B4B079B4C7ECA70D04E3F947A964B45=(CurveTable=None,RowName=\"\")),Duration_29_7F8704364211410D0930AD8AB240975B=(Source_10_0C1CA74C4C120C42C1F857BD53F0A76F=NewEnumerator0,Value_5_90E89AB144D6F3B57A2FB59966A03498=0.000000,CurveTable_11_2B4B079B4C7ECA70D04E3F947A964B45=(CurveTable=None,RowName=\"\")),DurationPolicy_32_683FC34B46CBA1C769699589F12C9837=NewEnumerator1,ExpirationPolicy_36_54D3E72548F23CD877ABE988E2FC308D=NewEnumerator0)" false "0.000000,0.000000,0.000000"))
    (else
      (Default|RemoveEffectbyClass (Variables|Default|GetAbilityManager) "/Game/AbilitySystem/Effects/ShieldRegeneration.ShieldRegeneration_C"))))

(event Custom|HandleHealthRegeneration
  (bind _health (Variables|Default|GetHealth))
  (if (< (Variables|/Game/AbilitySystem/BP_Attribute.BP_Attribute_C|GetCurrentValue (Variables|Default|GetHealth)) (|(RealValue-(RealValue*BlockedValue)) (Variables|/Game/AbilitySystem/BP_Attribute.BP_Attribute_C|GetRealValue _health) (Variables|/Game/AbilitySystem/BP_Attribute.BP_Attribute_C|GetBlockedValue _health)))
    (Default|ApplyEffect (Variables|Default|GetAbilityManager) (Utilities|Struct|MakeS_EffectData "/Game/AbilitySystem/Effects/HealthRegeneration.HealthRegeneration_C" 1 0 false "(Tick_17_40755E2C4DCAD94CF3DBA2AECC805C15=(Source_10_0C1CA74C4C120C42C1F857BD53F0A76F=NewEnumerator0,Value_5_90E89AB144D6F3B57A2FB59966A03498=0.000000,CurveTable_11_2B4B079B4C7ECA70D04E3F947A964B45=(CurveTable=None,RowName=\"\")),ChanceToApply_19_3C8E08B246FF3BA8A2CDA8A8D9F764C6=(Source_10_0C1CA74C4C120C42C1F857BD53F0A76F=NewEnumerator0,Value_5_90E89AB144D6F3B57A2FB59966A03498=0.000000,CurveTable_11_2B4B079B4C7ECA70D04E3F947A964B45=(CurveTable=None,RowName=\"\")),Duration_29_7F8704364211410D0930AD8AB240975B=(Source_10_0C1CA74C4C120C42C1F857BD53F0A76F=NewEnumerator0,Value_5_90E89AB144D6F3B57A2FB59966A03498=0.000000,CurveTable_11_2B4B079B4C7ECA70D04E3F947A964B45=(CurveTable=None,RowName=\"\")),DurationPolicy_32_683FC34B46CBA1C769699589F12C9837=NewEnumerator1,ExpirationPolicy_36_54D3E72548F23CD877ABE988E2FC308D=NewEnumerator0)" false "0.000000,0.000000,0.000000"))
    (else
      (Default|RemoveEffectbyClass (Variables|Default|GetAbilityManager) "/Game/AbilitySystem/Effects/HealthRegeneration.HealthRegeneration_C"))))

(event Custom|HandleEnergyRegeneration
  (bind _energy (Variables|Default|GetEnergy))
  (if (< (Variables|/Game/AbilitySystem/BP_Attribute.BP_Attribute_C|GetCurrentValue (Variables|Default|GetEnergy)) (|(RealValue-(RealValue*Blocked)) (Variables|/Game/AbilitySystem/BP_Attribute.BP_Attribute_C|GetRealValue _energy) (Variables|/Game/AbilitySystem/BP_Attribute.BP_Attribute_C|GetBlockedValue _energy)))
    (Default|ApplyEffect (Variables|Default|GetAbilityManager) (Utilities|Struct|MakeS_EffectData "/Game/AbilitySystem/Effects/EnergyRegeneration.EnergyRegeneration_C" 1 0 false "(Tick_17_40755E2C4DCAD94CF3DBA2AECC805C15=(Source_10_0C1CA74C4C120C42C1F857BD53F0A76F=NewEnumerator0,Value_5_90E89AB144D6F3B57A2FB59966A03498=0.000000,CurveTable_11_2B4B079B4C7ECA70D04E3F947A964B45=(CurveTable=None,RowName=\"\")),ChanceToApply_19_3C8E08B246FF3BA8A2CDA8A8D9F764C6=(Source_10_0C1CA74C4C120C42C1F857BD53F0A76F=NewEnumerator0,Value_5_90E89AB144D6F3B57A2FB59966A03498=0.000000,CurveTable_11_2B4B079B4C7ECA70D04E3F947A964B45=(CurveTable=None,RowName=\"\")),Duration_29_7F8704364211410D0930AD8AB240975B=(Source_10_0C1CA74C4C120C42C1F857BD53F0A76F=NewEnumerator0,Value_5_90E89AB144D6F3B57A2FB59966A03498=0.000000,CurveTable_11_2B4B079B4C7ECA70D04E3F947A964B45=(CurveTable=None,RowName=\"\")),DurationPolicy_32_683FC34B46CBA1C769699589F12C9837=NewEnumerator1,ExpirationPolicy_36_54D3E72548F23CD877ABE988E2FC308D=NewEnumerator0)" false "0.000000,0.000000,0.000000"))
    (else
      (Default|RemoveEffectbyClass (Variables|Default|GetAbilityManager) "/Game/AbilitySystem/Effects/EnergyRegeneration.EnergyRegeneration_C"))))

(event Custom|HandleManaRegeneration
  (bind _mana (Variables|Default|GetMana))
  (if (< (Variables|/Game/AbilitySystem/BP_Attribute.BP_Attribute_C|GetCurrentValue (Variables|Default|GetMana)) (|(RealValue-(RealValue*Blocked)) (Variables|/Game/AbilitySystem/BP_Attribute.BP_Attribute_C|GetRealValue _mana) (Variables|/Game/AbilitySystem/BP_Attribute.BP_Attribute_C|GetBlockedValue _mana)))
    (Default|ApplyEffect (Variables|Default|GetAbilityManager) (Utilities|Struct|MakeS_EffectData "/Game/AbilitySystem/Effects/ManaRegeneration.ManaRegeneration_C" 1 0 false "(Tick_17_40755E2C4DCAD94CF3DBA2AECC805C15=(Source_10_0C1CA74C4C120C42C1F857BD53F0A76F=NewEnumerator0,Value_5_90E89AB144D6F3B57A2FB59966A03498=0.000000,CurveTable_11_2B4B079B4C7ECA70D04E3F947A964B45=(CurveTable=None,RowName=\"\")),ChanceToApply_19_3C8E08B246FF3BA8A2CDA8A8D9F764C6=(Source_10_0C1CA74C4C120C42C1F857BD53F0A76F=NewEnumerator0,Value_5_90E89AB144D6F3B57A2FB59966A03498=0.000000,CurveTable_11_2B4B079B4C7ECA70D04E3F947A964B45=(CurveTable=None,RowName=\"\")),Duration_29_7F8704364211410D0930AD8AB240975B=(Source_10_0C1CA74C4C120C42C1F857BD53F0A76F=NewEnumerator0,Value_5_90E89AB144D6F3B57A2FB59966A03498=0.000000,CurveTable_11_2B4B079B4C7ECA70D04E3F947A964B45=(CurveTable=None,RowName=\"\")),DurationPolicy_32_683FC34B46CBA1C769699589F12C9837=NewEnumerator1,ExpirationPolicy_36_54D3E72548F23CD877ABE988E2FC308D=NewEnumerator0)" false "0.000000,0.000000,0.000000"))
    (else
      (Default|RemoveEffectbyClass (Variables|Default|GetAbilityManager) "/Game/AbilitySystem/Effects/ManaRegeneration.ManaRegeneration_C"))))