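; Player controller for the Ability System that sets up the pawn's managers and the display widget and handles hotkeys.
; BeginPlay initializes the equipment manager before the ability manager, reaching both through pawn messages, then the quick-slot manager.
; Keys drive interaction, cast cancelling, save/load, quitting, menus and target-data inspection; tooltips are lazily created and reused.
; The F inspector uses a HUD reference whose creation code never runs.
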(event EventUpdateAbilityQuickSlotHotkeys
  (Default|UpdateQuickSlotHotkeys (Variables|Default|GetAbilityQuickSlotManager)))

(event EventBeginPlay
  (bind _manager (Class|BIAbilitySystemActor|GetAbilityManager(Message) (Pawn|GetControlledPawn)))
  (Variables|Default|SetAbilityManager _manager)
  (bind _manager_2 (Class|BIAbilityEquipmentActor|GetEquipmentManagerA(Message) (Pawn|GetControlledPawn)))
  (Variables|Default|SetEquipmentManager _manager_2)
  (Default|Initialize (Variables|Default|GetEquipmentManager)) ; initialize before Ability Manager
  (Class|BIAbilitySystemActor|InitializeAbilityManager(Message) (Pawn|GetControlledPawn))
  (Default|Initialize (Variables|Default|GetAbilityQuickSlotManager))
  (bind _returnvalue (UserInterface|CreateWidget "/Game/MapUi/WBP_Display.WBP_Display_C"))
  (Variables|Default|SetMy_Hud _returnvalue)
  (UserInterface|Viewport|AddtoViewport (Variables|Default|GetMy_Hud) 0))

(event EventShowSystemNotificationA
  (params (Text :type Text))
  (bind _returnvalue (UserInterface|CreateWidget "/Game/AbilitySystem/GUI/NotificationSystem/WBP_SystemNotification.WBP_SystemNotification_C" 0 Text))
  (UserInterface|Viewport|AddtoViewport _returnvalue 10))

(event EventToggleHUDVisibilityA
  (params (IsVisible :type Boolean))
  (Widget|SetVisibility (Variables|Default|GetMy_Hud) (select IsVisible "Visible" "Hidden")))

(fn ConstructionScript)

(event Input|KeyboardEvents|V
  (params (Key :type Key%20Structure))
  (:Pressed
    (if (Game|Player|IsInputKeyDown "LeftShift")
      (bind _outactors (Collision|SphereOverlapActors (Transformation|GetActorLocation (Pawn|GetControlledPawn)) 5e+03 (Utilities|Array|MakeArray "ObjectTypeQuery3" "ObjectTypeQuery1" "ObjectTypeQuery2" "ObjectTypeQuery4") 0))
      (for _array_element _outactors
        (Utilities|IsValid (Actor|GetComponentbyClass _array_element "/Game/AbilitySystem/GUI/AbilitySystem/WC_TargetData.WC_TargetData_C")
          (:Is%20Valid
            (Default|Destroy (Actor|GetComponentbyClass _array_element "/Game/AbilitySystem/GUI/AbilitySystem/WC_TargetData.WC_TargetData_C")))))
      (else
        (Class|BIInteractionAbilityActor|ShowDatainWorld(Message) (.HitActor (Collision|BreakHitResult (.HitResult (Game|Player|GetHitResultUnderCursorbyChannel "TraceTypeQuery1" true)))))))))

(event Input|KeyboardEvents|R
  (params (Key :type Key%20Structure))
  (:Pressed
    (Variables|Default|GetInteractionTarget
      (:then
        (Default|TryActivateAbility (Variables|Default|GetAbilityManager) "/Game/AbilitySystem/Abilities/Overall_Interaction.Overall_Interaction_C"))
      (:else))))

(event Input|KeyboardEvents|K
  (params (Key :type Key%20Structure))
  (:Pressed
    (Class|BIGameAbilityGI|SaveGameA(Message) (Game|GetGameInstance) "AbilitySystem")))

(event Input|KeyboardEvents|L
  (params (Key :type Key%20Structure))
  (:Pressed
    (Class|BIGameAbilityGI|LoadGameA(Message) (Game|GetGameInstance) "AbilitySystem")))

(event Input|KeyboardEvents|Escape
  (params (Key :type Key%20Structure))
  (:Pressed
    (Game|QuitGame 0 "Quit" false)))

(event Input|KeyboardEvents|G
  (params (Key :type Key%20Structure))
  (:Pressed
    (bind _returnvalue (UserInterface|CreateWidget "/Game/AbilitySystem/GUI/WBP_GameModes.WBP_GameModes_C"))
    (UserInterface|Viewport|AddtoViewport _returnvalue 10)))

(event Input|KeyboardEvents|Tab
  (params (Key :type Key%20Structure))
  (:Pressed
    (Default|CancelCurrentlyCastedAbility (Variables|Default|GetAbilityManager))))

(event Input|KeyboardEvents|F
  (params (Key :type Key%20Structure))
  (:Pressed
    (Default|Initialize (Variables|/Game/AbilitySystem/GUI/WBP_HUD_Ability.WBP_HUD_Ability_C|GetWBP_TargetData (Variables|Default|GetHUD)) (.HitActor (Collision|BreakHitResult (.HitResult (Game|Player|GetHitResultUnderCursorbyChannel "TraceTypeQuery1" true)))))))

(event Input|KeyboardEvents|C
  (params (Key :type Key%20Structure))
  (:Pressed
    (Variables|Default|GetCharacterWindow
      (:then
        _)
      (:else
        (bind _returnvalue (UserInterface|CreateWidget "/Game/AbilitySystem/GUI/WBP_CharacterWindow_Ability.WBP_CharacterWindow_Ability_C"))
        (Variables|Default|SetCharacterWindow _returnvalue)))
    (UserInterface|Viewport|AddtoViewport (Variables|Default|GetCharacterWindow) 0)
    (CallFunction|ToggleHUDVisibilityA false)))

(fn GenerateAbilityTooltip
  (params (Ability :type BP%20Ability%20Object%20Reference))
  (Variables|Default|GetAbilityTooltip
    (:then
      _)
    (:else
      (bind _returnvalue (UserInterface|CreateWidget "/Game/AbilitySystem/GUI/AbilitySystem/WBP_AbilityTooltip.WBP_AbilityTooltip_C"))
      (Variables|Default|SetAbilityTooltip _returnvalue)))
  (Default|Update (Variables|Default|GetAbilityTooltip) Ability)
  (return (Variables|Default|GetAbilityTooltip)))

(fn GenerateEffectTooltip
  (params (Effect :type BP%20Effect%20Object%20Reference))
  (Variables|Default|GetEffectTooltip
    (:then
      _)
    (:else
      (bind _returnvalue (UserInterface|CreateWidget "/Game/AbilitySystem/GUI/AbilitySystem/WBP_EffectTooltip.WBP_EffectTooltip_C"))
      (Variables|Default|SetEffectTooltip _returnvalue)))
  (Default|Update (Variables|Default|GetEffectTooltip) Effect)
  (return (Variables|Default|GetEffectTooltip)))

(fn GetInteractionTargetA
  (return (Variables|Default|GetInteractionTarget)))