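; BP_Skill02 is a short-lived skill actor that plays the BM_Combo02 montage on the player's mesh.
; On BeginPlay it runs the parent logic, then starts the montage on the skeletal mesh of its BPPlayer reference.
; The actor destroys itself when the montage completes, with no handling for interruption.
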(event EventBeginPlay
  (|CallParentFunction)
  (Animation|Montage|PlayMontage (Variables|/Script/Engine.Character|GetMesh (.BP_Player (Variables|Default|GetBP_Player))) "/Game/Characters/ABP_ADA/Animation/Skill/BM_Combo02.BM_Combo02"
    (:OnCompleted
      (Actor|DestroyActor))))

(event Collision|EventActorBeginOverlap
  (params (OtherActor :type Actor%20Object%20Reference))
  (|CallParentFunction OtherActor) ; This node is disabled and will not be called.\nDrag off pins to build functionality.
)

(event EventTick
  (params (DeltaSeconds :type Float%20%28single-precision%29))
  (|CallParentFunction DeltaSeconds) ; This node is disabled and will not be called.\nDrag off pins to build functionality.
)

(fn ConstructionScript
  (|CallParentFunction))