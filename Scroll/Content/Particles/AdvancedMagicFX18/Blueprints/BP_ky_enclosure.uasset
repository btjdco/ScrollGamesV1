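; Magic enclosure effect actor that exposes a ColorIn setting to tint its FX particle component.
; The construction script creates dynamic material instances for the first two FX material slots, sets their "incolor" parameter, and passes the colour to the particle system's "inColor" vector parameter.
; BeginPlay recreates both material instances and reapplies the colour to them, leaving the particle parameter to the construction script.
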(event EventBeginPlay
  ;[1 1 1] core color control
  (bind _returnvalue (Rendering|Material|CreateDynamicMaterialInstance (Variables|Default|GetFX) 0 0 "None" :!class /Script/Engine.PrimitiveComponent))
  (bind _returnvalue_2 (Rendering|Material|CreateDynamicMaterialInstance (Variables|Default|GetFX) 1 0 "None" :!class /Script/Engine.PrimitiveComponent))
  (Rendering|Material|SetVectorParameterValue _returnvalue "incolor" (Variables|Default|GetcolorIn) :!class /Script/Engine.MaterialInstanceDynamic)
  (|CallParentFunction))

(event Collision|EventActorBeginOverlap
  (params (OtherActor :type Actor%20Object%20Reference))
  (|CallParentFunction 0))

(event EventTick
  (params (DeltaSeconds :type Float%20%28single-precision%29))
  (|CallParentFunction 0.0))

(fn ConstructionScript
  (bind _colorin (Variables|Default|GetcolorIn))
  (|CallParentFunction)
  ;[1 1 1] core color control
  (bind _returnvalue (Rendering|Material|CreateDynamicMaterialInstance (Variables|Default|GetFX) 0 0 "None" :!class /Script/Engine.PrimitiveComponent))
  (bind _returnvalue_2 (Rendering|Material|CreateDynamicMaterialInstance (Variables|Default|GetFX) 1 0 "None" :!class /Script/Engine.PrimitiveComponent))
  (Rendering|Material|SetVectorParameterValue _returnvalue "incolor" _colorin :!class /Script/Engine.MaterialInstanceDynamic)
  (Effects|Components|ParticleSystem|SetVectorParameter (Variables|Default|GetFX) "inColor" (Math|Conversions|ToVector(LinearColor) _colorin)))