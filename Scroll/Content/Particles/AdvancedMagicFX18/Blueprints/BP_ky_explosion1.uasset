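; BP_ky_explosion1 is an explosion effect Blueprint from the AdvancedMagicFX18 particle pack with an adjustable secondary color.
; Its construction script converts the ColorSub variable to a vector and passes it to the FX component's "colorSub" parameter.
; The event graph holds only disabled default events, so the Blueprint adds no runtime logic.
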(event EventBeginPlay
  (|CallParentFunction))

(event Collision|EventActorBeginOverlap
  (params (OtherActor :type Actor%20Object%20Reference))
  (|CallParentFunction 0))

(event EventTick
  (params (DeltaSeconds :type Float%20%28single-precision%29))
  (|CallParentFunction 0.0))

(fn ConstructionScript
  ;[1 1 1] color control
  (|CallParentFunction)
  (Effects|Components|ParticleSystem|SetVectorParameter (Variables|Default|GetFX) "colorSub" (Math|Conversions|ToVector(LinearColor) (Variables|Default|GetcolorSub))))