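; Projectile actor that damages any Character it hits, with a fireball explosion at the impact.
; On BeginPlay it rotates its starting velocity to the actor's facing, and a Life timeline gradually shrinks it.
; When the timeline ends, it toggles the effect off and briefly delays destruction so particles can fade.
; A Character hit destroys the bullet and adds an impulse to the mesh if it is simulating physics.
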(event Collision|EventHit
  (params (MyComp :type Primitive%20Component%20Object%20Reference) (Other :type Actor%20Object%20Reference) (OtherComp :type Primitive%20Component%20Object%20Reference) (bSelfMoved :type Boolean) (HitLocation :type Vector :default "0, 0, 0") (HitNormal :type Vector :default "0, 0, 0") (NormalImpulse :type Vector :default "0, 0, 0") (Hit :type Hit%20Result%20Structure%20%28by%20ref%29))
  (bind _ascharacter (Utilities|Casting|CastToCharacter Other))
  (Game|Damage|ApplyDamage _ascharacter 1e+01 (Game|GetInstigatorController) 0)
  (Effects|SpawnEmitteratLocation "/Game/UI_Kit/Showcase/Particles/P_Explosion_Fireball.P_Explosion_Fireball" (Transformation|GetActorLocation))
  (Actor|DestroyActor)
  (if (Physics|IsSimulatingPhysics (Variables|/Script/Engine.Character|GetMesh _ascharacter) "None")
    (Physics|AddImpulse (Variables|/Script/Engine.Character|GetMesh _ascharacter) (* HitNormal -5e+04) "None" false)))

(event EventBeginPlay
  (Variables|/Script/Engine.MovementComponent|SetVelocity (Variables|Default|GetProjectileMovement) (Math|Vector|RotateVector (Variables|Default|GetStarting%20Velocity) (Transformation|GetActorRotation))) ; Set the speed/direction of the projectile
  (bind _scale (Timeline|Life Play) ; Timeline blends from 1 to 0.15
    (:Update
      (Transformation|SetActorRelativeScale3D (* (Math|Vector|MakeVector 1.0 1.0 1.0) _scale)) ; Gradually shrink the actor
    )
    (:Finished
      (Components|Activation|ToggleActive (Variables|Default|GetEffect)) ; Turn off effect to give particles a chance to fade instead of disappearing suddenly when the actor is destroyed
      (Utilities|FlowControl|Delay 0.1)
      (Actor|DestroyActor))))

(fn ConstructionScript)